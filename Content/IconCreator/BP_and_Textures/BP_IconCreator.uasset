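; BP_IconCreator is a capture rig that frames a skeletal mesh, static mesh or child actor for icon rendering.
; The construction script applies exposed meshes, transforms, light intensities and field of view, forcing skeletal LOD 0.
; It fills the scene capture's show-only lists with all BP_IconCreator actors and the Border component.
; AddToShowOnlyList adds the child actor and stops its skeletal mesh animations.
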(event Custom|AddToShowOnlyList
  (bind _childactor (Variables|Default|GetChildActor))
  (bind _childactor_2 (Variables|/Script/Engine.ChildActorComponent|GetChildActor _childactor))
  (Utilities|IsValid _childactor_2
    (:Is%20Valid
      (Utilities|Array|Add (Variables|/Script/Engine.SceneCaptureComponent|GetShowOnlyActors (Variables|Default|GetSceneCaptureComponent2D)) _childactor_2)
      (for _array_element (Actor|GetComponentsByClass _childactor_2 "/Script/Engine.SkeletalMeshComponent")
        (Audio|Components|Audio|Stop _array_element)))))

(fn ConstructionScript
  (bind _scenecapturecomponent2d (Variables|Default|GetSceneCaptureComponent2D))
  (Class|SkinnedMeshComponent|SetSkeletalMesh (Variables|Default|GetSkeletalMesh) (Variables|Default|SkeletalMesh|GetSkeletalM) true)
  (Components|StaticMesh|SetStaticMesh (Variables|Default|GetStaticMesh) (Variables|Default|StaticMesh|GetStaticM))
  (Variables|/Script/Engine.SceneCaptureComponent2D|SetFOVAngle (Variables|Default|GetSceneCaptureComponent2D) (Variables|Default|Zoom|GetFieldOfView))
  (Rendering|Components|Light|SetIntensity (Variables|Default|GetExtraLight1) (Variables|Default|ExtraLight|GetExtraLight_01))
  (Rendering|Components|Light|SetIntensity (Variables|Default|GetExtraLight2) (Variables|Default|ExtraLight|GetExtraLight_02))
  (Rendering|Components|Light|SetIntensity (Variables|Default|GetExtraLight3) (Variables|Default|ExtraLight|GetExtraLight_03))
  (Rendering|Components|Light|SetIntensity (Variables|Default|GetExtraLight4) (Variables|Default|ExtraLight|GetExtraLight_04))
  (Rendering|Components|Light|SetIntensity (Variables|Default|GetSpotLight1) (Variables|Default|MainLight|GetMainLight1))
  (Rendering|Components|Light|SetIntensity (Variables|Default|GetSpotLight2) (Variables|Default|MainLight|GetMainLight2))
  (Transformation|SetRelativeTransform (Variables|Default|GetSkeletalMesh) (Math|Transform|MakeTransform (Variables|Default|SkeletalMesh|GetSkeletalM_Loc) (Variables|Default|SkeletalMesh|GetSkeletalM_Rot) (Variables|Default|SkeletalMesh|GetSkeletalM_Scale)) false false)
  (Class|SkinnedMeshComponent|SetMinLOD (Variables|Default|GetSkeletalMesh))
  (Transformation|SetRelativeTransform (Variables|Default|GetStaticMesh) (Math|Transform|MakeTransform (Variables|Default|StaticMesh|GetStaticM_Loc) (Variables|Default|StaticMesh|GetStaticM_Rot) (Variables|Default|StaticMesh|GetStaticM_Scale)) false false)
  (bind _outactors (Actor|GetAllActorsOfClass "BP_IconCreator_C"))
  (for _array_element _outactors
    (Utilities|Array|Add (Variables|/Script/Engine.SceneCaptureComponent|GetShowOnlyActors (Variables|Default|GetSceneCaptureComponent2D)) _array_element)
    (Rendering|SceneCapture|ShowOnlyActorComponents _scenecapturecomponent2d _array_element))
  (Rendering|SceneCapture|ShowOnlyComponent _scenecapturecomponent2d (Variables|Default|GetBorder)))