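; Parent enemy Blueprint providing shared combat, movement speed, health bar and death handling, with placeholder day/night hooks bound to BP_TimeOfDay.
; Construction hands the child-actor weapon to CombatComponent, while Tick shows the health bar near the player.
; CombatComponent's death event ragdolls the mesh, updates the AI blackboard, spawns ground-traced loot, advances matching bounty quests, releases target lock, then destroys the actor.
; Attacks time their IsAttacking flag from the AnimBP's sequence length.
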(event Custom|Walk
  ;[1 1 1] Set Walk / Run Speed
  (Variables|/Script/Engine.CharacterMovementComponent|SetMaxWalkSpeed (Variables|Character|GetCharacterMovement) (Variables|Default|GetWalkSpeed)))

(event Custom|Run
  ;[1 1 1] Set Walk / Run Speed
  (Variables|/Script/Engine.CharacterMovementComponent|SetMaxWalkSpeed (Variables|Character|GetCharacterMovement) (Variables|Default|GetRunSpeed)))

(event Custom|NightBehavior
  ;[1 1 1] Day / Night Behavior
  (if (Variables|Default|GetNightActive?)
    _))

(event Custom|DayBehavior
  ;[1 1 1] Day / Night Behavior
  (if (Variables|Default|GetNightActive?)
    _))

(event Custom|AttackPlayer
  ;[1 0.2584 0.2285] Attack the Player
  (Variables|Default|SetIsAttacking true)
  (bind _asenemy_anim_bp_parent (Utilities|Casting|CastToEnemy_AnimBP_Parent (Components|SkeletalMesh|GetAnimInstance (Variables|Character|GetMesh)))
    (:then
      (Utilities|FlowControl|Delay (Variables|/Script/Engine.AnimSequenceBase|GetSequenceLength (Variables|/Game/Blueprints/Characters/Enemies/Enemy_AnimBP_Parent.Enemy_AnimBP_Parent_C|GetAttackSequence _asenemy_anim_bp_parent))))
    (:CastFailed
      (Utilities|FlowControl|Delay 1.0)))
  (Variables|Default|SetIsAttacking false))

(event EventTargetLockON
  ;[1 1 1] Highlight Enemy when TargetLocked
  (bind _isa (Utilities|FlowControl|FlipFlop)
    (:A
      (Variables|Default|SetIsLockedON _isa))
    (:B
      (Variables|Default|SetIsLockedON _isa)))
  (Development|SetHiddeninGame (Variables|Default|GetCone) (not (Variables|Default|GetIsLockedON)) false))

(event EventTick
  (params (DeltaSeconds :type Float%20%28single-precision%29))
  ;[1 1 1] Update
  (if (not (Variables|Default|GetisDead))
    (CallFunction|DisplayHealthbarwheninRange)))

(event EventBeginPlay
  ;[1 1 1] Initialization
  (|CallParentFunction)
  (bind _output_get (Variables|Default|SetHealthbarWidget (.AsEnemy%20Healthbar (Utilities|Casting|CastToEnemyHealthbar (UserInterface|GetUserWidgetObject (Variables|Default|GetEnemyHealthbar))))))
  (Variables|/Game/Blueprints/Characters/Enemies/EnemyHealthbar.EnemyHealthbar_C|SetEnemyActor _output_get self)
  (Variables|Default|SetPlayerRef (.AsMain%20Character%20BP (Utilities|Casting|CastToMainCharacter_BP (Game|GetPlayerCharacter 0))))
  (bind _returnvalue (Actor|GetActorOfClass "/Game/Blueprints/BP_TimeOfDay.BP_TimeOfDay_C"))
  (bind _output_get_2 (Variables|Default|SetTimeOfDayRef _returnvalue))
  (EventDispatchers|BindEventtoNightTime _output_get_2 (delegate Custom|NightBehavior))
  (EventDispatchers|BindEventtoDayTime _output_get_2 (delegate Custom|DayBehavior))
  (EventDispatchers|BindEventtoDeath (Variables|Default|GetCombatComponent) (delegate EventOnDeath)))

(event EventOnDeath
  (bind _mesh (Variables|Character|GetMesh))
  ;[1 1 1] Enemy dies
  (Class|SkeletalMeshComponent|SetAllBodiesSimulatePhysics _mesh true)
  (Class|SkeletalMeshComponent|SetPhysicsBlendWeight _mesh 1.0)
  (bind _output_get (Variables|Default|SetisDead true))
  (AI|Components|Blackboard|SetValueasBool (AI|GetBlackboard (.AsEnemy%20AIController (Utilities|Casting|CastToEnemyAIController (Pawn|GetController)))) (Utilities|Name|MakeLiteralName "IsDead") _output_get)
  (Collision|SetCollisionEnabled (Variables|Default|GetCapsuleComponent) "NoCollision")
  (CallFunction|SpawnLoot)
  (CallFunction|UpdateBountyQuests)
  (if (Variables|Default|GetIsLockedON)
    (Default|TargetKilled (Variables|/Game/Blueprints/Characters/MainCharacter/MainCharacter_BP.MainCharacter_BP_C|GetTargetLockComponent (Variables|Default|GetPlayerRef))))
  (Audio|PlaySoundatLocation (Variables|Default|GetDeathSound) (Transformation|GetActorLocation) "0, 0, 0" 1.0 1.0 0.0 0 0 0)
  (Rendering|SetVisibility (Variables|Default|GetCone) false false)
  (Utilities|FlowControl|Delay 3.0)
  (Actor|DestroyActor))

(fn ConstructionScript
  (Variables|Default|SetSpawnOrigin (Transformation|GetActorLocation))
  (bind _output_get (Variables|/Game/Blueprints/Characters/CombatBP/CombatComponent.CombatComponent_C|SetActiveWeapon (Variables|Default|GetCombatComponent) (.AsItem%20Weapon%20Parent (Utilities|Casting|CastToItem_WeaponParent (Variables|/Script/Engine.ChildActorComponent|GetChildActor (Variables|Default|GetWeapon))))))
  (Variables|/Game/Blueprints/UI/Interactables/BP_Interactable_Parent_Actor.BP_Interactable_Parent_Actor_C|SetIsInteractable _output_get false)
  (Collision|SetCollisionEnabled (Variables|/Game/Blueprints/UI/Interactables/BP_Interactable_StaticActor.BP_Interactable_StaticActor_C|GetInteractionMesh _output_get) "NoCollision"))

(fn DistancefromPlayerCheck
  (return (Transformation|GetDistanceTo (Game|GetPlayerCharacter 0))))

(fn UpdateBountyQuests
  (bind _asmain_character_bp (Utilities|Casting|CastToMainCharacter_BP (Game|GetPlayerCharacter 0)))
  (for _array_element (Variables|/Game/Blueprints/Quests/BP_QuestListComponent.BP_QuestListComponent_C|GetAllQuests (Variables|/Game/Blueprints/Characters/MainCharacter/MainCharacter_BP.MainCharacter_BP_C|GetQuestList _asmain_character_bp))
    (for _array_element_2 (Variables|/Game/Blueprints/Quests/BP_QuestParent.BP_QuestParent_C|GetCurrentQuestGoals _array_element)
      (bind _asbp_quest_goal_bounty (Utilities|Casting|CastToBP_QuestGoal_Bounty _array_element_2))
      (if (== (Variables|/Game/Blueprints/Quests/BP_QuestGoal_Bounty.BP_QuestGoal_Bounty_C|GetEnemyType _asbp_quest_goal_bounty) (Utilities|GetClass self))
        (Default|IncrementCurrentBounty _asbp_quest_goal_bounty)
        (Default|Update _asbp_quest_goal_bounty)))))

(fn DisplayHealthbarwheninRange
  (bind _enemyhealthbar (Variables|Default|GetEnemyHealthbar))
  (if (< (Transformation|GetDistanceTo (Variables|Default|GetPlayerRef)) 1e+03)
    (Rendering|SetVisibility _enemyhealthbar true false)
    (else
      (Rendering|SetVisibility _enemyhealthbar false false))))

(fn SpawnLoot
  (bind _returnvalue (Transformation|GetActorLocation))
  (bind _itemclassdrop (Variables|Default|GetItemClassDrop)
    (:then
      (bind _outhit (Collision|LineTraceByChannel (+ _returnvalue "0, 0,50.000000") (- _returnvalue "0, 0,200.000000") "TraceTypeQuery1" false 0 "None"))
      (bind _returnvalue_2 (Game|SpawnActorfromClass _itemclassdrop (Math|Transform|MakeTransform (.Location (Collision|BreakHitResult _outhit)) (Math|Rotator|MakeRotator 0.0 0.0 (* (Math|Random|RandomFloat) 3.6e+02)) "1,1,1") "Undefined" 0 false true 0))
      (return _returnvalue_2))
    (:else)))