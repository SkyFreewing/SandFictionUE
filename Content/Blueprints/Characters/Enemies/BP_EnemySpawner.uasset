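; Enemy spawner placed in the level that keeps one enemy of a set class alive during either night or day.
; It binds to BP_TimeOfDay's night and day events, and the NightEnemy flag decides which phase spawns and which despawns.
; Spawning destroys any previous enemy, then creates the pawn with its behavior tree at the spawner's location.
; An editor-time label and red or green sphere show the setup, both removed at BeginPlay.
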(event Custom|NightEvent
  (if (Variables|Default|GetNightEnemy)
    (CallFunction|Spawn)
    (else
      (CallFunction|Despawn))))

(event Custom|DayEvent
  (if (Variables|Default|GetNightEnemy)
    (CallFunction|Despawn)
    (else
      (CallFunction|Spawn))))

(event EventBeginPlay
  (Components|DestroyComponent (Variables|Default|GetSphere))
  (bind _returnvalue (Actor|GetActorOfClass "/Game/Blueprints/BP_TimeOfDay.BP_TimeOfDay_C"))
  (bind _output_get (Variables|Default|SetTimeBP _returnvalue))
  (EventDispatchers|BindEventtoNightTime _output_get (delegate Custom|NightEvent))
  (EventDispatchers|BindEventtoDayTime _output_get (delegate Custom|DayEvent)))

(fn ConstructionScript
  (bind _sphere (Variables|Default|GetSphere))
  (Rendering|Components|TextRender|SetText (Variables|Default|GetTextRender) (.Name (Utilities|GetClassDefaults (Variables|Default|GetEnemyClass))))
  (if (Variables|Default|GetNightEnemy)
    (Rendering|Material|CreateDynamicMaterialInstance _sphere 0 "/Game/Materials/Debug/MI_RedDebug.MI_RedDebug" "None" :!class /Script/Engine.PrimitiveComponent)
    (else
      (Rendering|Material|CreateDynamicMaterialInstance _sphere 0 "/Game/Materials/Debug/MI_GreenDebug.MI_GreenDebug" "None" :!class /Script/Engine.PrimitiveComponent))))

(fn Spawn
  (CallFunction|Despawn)
  (bind _returnvalue (AI|SpawnAIFromClass (Variables|Default|GetEnemyClass) (Variables|Default|GetEnemyBT) (Transformation|GetActorLocation) "0, 0, 0" false))
  (Variables|Default|SetSpawnedEnemy _returnvalue)
  (Development|PrintString "Enemy Spawned"))

(fn Despawn
  (bind _spawnedenemy (Variables|Default|GetSpawnedEnemy)
    (:then
      (Actor|DestroyActor _spawnedenemy))
    (:else
      _))
  (return))