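; BP_GameCharacter_Humans is a human character Blueprint containing eye-blink logic that is currently not triggered.
; The RandomBlink update feeds a DoOnce gate that plays the BlinkAnim timeline and resets after a random delay of a few seconds.
; BlinkAnim drives the left and right blink morph targets through the mesh's anim instance.
; Nothing starts either chain, and the construction script only calls its parent.
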(fn ConstructionScript
  (|CallParentFunction))