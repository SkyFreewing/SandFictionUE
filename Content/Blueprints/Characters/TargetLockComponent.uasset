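; Player target-lock component that locks the camera onto an Enemy_ParentBP and can turn the character toward it.
; Target selection line-traces enemies in range and scores them by angle from camera center, with pitch weighted by distance.
; While locked, a gated Tick updates control rotation and checks range and line of sight, using a retriggerable delay as grace period.
; Mouse wheel switches to the closest left or right enemy, and kills trigger delayed retargeting.
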(event Custom|New%20Target%20after%20Old%20dies
  (bind _followcamera (Variables|Default|GetFollowCamera))
  (bind _returnvalue (Transformation|GetWorldLocation _followcamera))
  ;[1 1 1] Target Lock
  (Utilities|FlowControl|Delay 0.2)
  (Variables|Default|SetOffCenter 3.6e+02)
  (Variables|Default|SetStartVector (Math|Vector|MakeVector (.x _returnvalue) (.y _returnvalue) (+ (.z _returnvalue) 2e+02)))
  (Variables|Default|SetClosesTargetDistance (Variables|Default|GetMinimumDistanceToEnable))
  (if (Variables|Default|GetTargetLocked)
    (Variables|Default|SetTargetLocked false)
    (bind _nearesttarget (Variables|Default|GetNearestTarget :!label _label)
      (:then
        (Class|CombatBPI|TargetLockON(Message) _nearesttarget)
        (Utilities|FlowControl|Gate true) ; enters at Toggle
      )
      (:else
        (Utilities|FlowControl|Gate true) ; enters at Toggle
      ))
    (else
      (bind _outactors (Actor|GetAllActorsOfClass "/Game/Blueprints/Characters/Enemies/Enemy_ParentBP.Enemy_ParentBP_C"))
      (for _array_element _outactors
        (Variables|Default|SetEnemyElement _array_element)
        (bind _outhit (Collision|LineTraceForObjects (Transformation|GetActorLocation (Components|GetOwner)) (Transformation|GetActorLocation (Variables|Default|GetEnemyElement)) (Utilities|Array|MakeArray "ObjectTypeQuery3") false 0 "None"))
        (if (== (Variables|Default|GetEnemyElement) (.HitActor (Collision|BreakHitResult _outhit)))
          (bind _distancefromplayer (Default|DistancefromPlayerCheck (Variables|Default|GetEnemyElement)))
          (Math|Float|CompareFloat _distancefromplayer (Variables|Default|GetMinimumDistanceToEnable)
            (:<
              (CallFunction|AngleCheck)
              (Utilities|FlowControl|DoOnce false
                (:Completed
                  (CallFunction|LockOff)))))))
      (if (< (Variables|Default|GetClosesTargetDistance) (Variables|Default|GetMinimumDistanceToEnable))
        (Variables|Default|SetTargetLocked true)
        (goto _label)))))

(event Custom|BreakLineOfSight
  ;[1 1 1] Lock off when Line of Sight to Enemy breaks
  (if (Variables|Default|GetTargetLocked)
    (bind _outactors (Actor|GetAllActorsOfClass "/Game/Blueprints/Characters/Enemies/Enemy_ParentBP.Enemy_ParentBP_C"))
    (bind _output_get (Variables|Default|SetEnemyArray _outactors))
    (bind _nearesttarget (Variables|Default|GetNearestTarget)
      (:then
        (Utilities|Array|RemoveItem _output_get _nearesttarget)
        (bind _outhit (Collision|LineTraceForObjects (Variables|Default|GetStartVector) (Transformation|GetWorldLocation (Variables|/Script/Engine.Character|GetCapsuleComponent (Variables|Default|GetNearestTarget))) (Utilities|Array|MakeArray "ObjectTypeQuery1" "ObjectTypeQuery2" "ObjectTypeQuery3") false (Variables|Default|GetEnemyArray) "None"))
        (if (== (Variables|Default|GetNearestTarget) (.HitActor (Collision|BreakHitResult _outhit)))
          (Utilities|FlowControl|RetriggerableDelay 2.0)
          (CallFunction|LockOff)))
      (:else
        (CallFunction|LockOff)))))

(event Custom|DistanceLockOff
  ;[1 1 1] Target Lock
  (if (Variables|Default|GetTargetLocked)
    (bind _distancefromplayer (Default|DistancefromPlayerCheck (Variables|Default|GetNearestTarget)))
    (if (not (< _distancefromplayer (Variables|Default|GetMinimumDistanceToEnable)))
      (Utilities|FlowControl|DoOnce false
        (:Completed
          (CallFunction|LockOff))))))

(event Custom|PlayerDiesLockOff
  ;[1 1 1] Lock Off when Player dies
)

(event Custom|MouseWheelUp
  (bind _nearesttarget (Variables|Default|GetNearestTarget))
  ;[1 1 1] Switch Enemy when Scrolling with Mouse Wheel
  (Variables|Default|SetSwapDirection 1)
  (if (Variables|Default|GetTargetLocked)
    (Class|CombatBPI|TargetLockON(Message) (Variables|Default|GetNearestTarget))
    (Variables|Default|SetClosesTargetDistance (Variables|Default|GetMinimumDistanceToEnable))
    (Variables|Default|SetCurrentTarget (Variables|Default|GetNearestTarget))
    (bind _outactors (Actor|GetAllActorsOfClass "/Game/Blueprints/Characters/Enemies/Enemy_ParentBP.Enemy_ParentBP_C"))
    (for _array_element _outactors
      (Variables|Default|SetEnemyElement _array_element)
      (bind _outhit (Collision|LineTraceForObjects (Variables|Default|GetStartVector) (Transformation|GetWorldLocation (Variables|/Game/Blueprints/Characters/Enemies/Enemy_ParentBP.Enemy_ParentBP_C|GetRayCollision (Variables|Default|GetEnemyElement))) (Utilities|Array|MakeArray "ObjectTypeQuery1" "ObjectTypeQuery2" "ObjectTypeQuery3") false (Utilities|Array|MakeArray (Variables|Default|GetCurrentTarget) _nearesttarget) "None"))
      (if (== (Variables|Default|GetEnemyElement) (.HitActor (Collision|BreakHitResult _outhit)))
        (switch int (Variables|Default|GetSwapDirection)
          (:0
            (CallFunction|EnemytoLeft))
          (:1
            (CallFunction|EnemytoRight)))))
    (Class|CombatBPI|TargetLockON(Message) _nearesttarget)))

(event Custom|MouseWheelDown
  (bind _nearesttarget (Variables|Default|GetNearestTarget))
  ;[1 1 1] Switch Enemy when Scrolling with Mouse Wheel
  (Variables|Default|SetSwapDirection 0)
  (if (Variables|Default|GetTargetLocked)
    (Class|CombatBPI|TargetLockON(Message) (Variables|Default|GetNearestTarget))
    (Variables|Default|SetClosesTargetDistance (Variables|Default|GetMinimumDistanceToEnable))
    (Variables|Default|SetCurrentTarget (Variables|Default|GetNearestTarget))
    (bind _outactors (Actor|GetAllActorsOfClass "/Game/Blueprints/Characters/Enemies/Enemy_ParentBP.Enemy_ParentBP_C"))
    (for _array_element _outactors
      (Variables|Default|SetEnemyElement _array_element)
      (bind _outhit (Collision|LineTraceForObjects (Variables|Default|GetStartVector) (Transformation|GetWorldLocation (Variables|/Game/Blueprints/Characters/Enemies/Enemy_ParentBP.Enemy_ParentBP_C|GetRayCollision (Variables|Default|GetEnemyElement))) (Utilities|Array|MakeArray "ObjectTypeQuery1" "ObjectTypeQuery2" "ObjectTypeQuery3") false (Utilities|Array|MakeArray (Variables|Default|GetCurrentTarget) _nearesttarget) "None"))
      (if (== (Variables|Default|GetEnemyElement) (.HitActor (Collision|BreakHitResult _outhit)))
        (switch int (Variables|Default|GetSwapDirection)
          (:0
            (CallFunction|EnemytoLeft))
          (:1
            (CallFunction|EnemytoRight)))))
    (Class|CombatBPI|TargetLockON(Message) _nearesttarget)))

(event Custom|Initialize%20Target%20Lock
  (params (FollowCamera :type Camera%20Component%20Object%20Reference) (CameraBoom :type Spring%20Arm%20Component%20Object%20Reference) (PlayerRef :type Main%20Character%20BP%20Object%20Reference))
  ;[1 1 1] Initialize
  (Variables|Default|SetFollowCamera FollowCamera)
  (Variables|Default|SetCameraBoom CameraBoom)
  (Variables|Default|SetPlayerRef PlayerRef))

(event Custom|LockOff
  ;[1 1 1] Target Lock
  (if (Variables|Default|GetTargetLocked)
    (Variables|Default|SetTargetLocked false)
    (bind _nearesttarget (Variables|Default|GetNearestTarget)
      (:then
        (Class|CombatBPI|TargetLockON(Message) _nearesttarget)
        (Utilities|FlowControl|Gate true) ; enters at Toggle
      )
      (:else
        (Utilities|FlowControl|Gate true) ; enters at Toggle
      ))))

(event Custom|TargetKilled
  ;[1 1 1] Target Lock
  (CallFunction|NewTargetAfterOldDies)
  (Variables|Default|SetTargetLocked false)
  (bind _nearesttarget (Variables|Default|GetNearestTarget)
    (:then
      (Class|CombatBPI|TargetLockON(Message) _nearesttarget)
      (Utilities|FlowControl|Gate true) ; enters at Toggle
    )
    (:else
      (Utilities|FlowControl|Gate true) ; enters at Toggle
    )))

(event Custom|EnemyToLeft
  (bind _cameraboom (Variables|Default|GetCameraBoom))
  (bind _enemyelement (Variables|Default|GetEnemyElement))
  (bind _currenttarget (Variables|Default|GetCurrentTarget))
  (bind _followcamera (Variables|Default|GetFollowCamera))
  (bind _returnvalue (Transformation|GetWorldTransform _cameraboom))
  (bind _returnvalue_2 (Transformation|GetWorldTransform _followcamera))
  (bind _rootcomponent (Variables|/Script/Engine.Actor|GetRootComponent _enemyelement))
  (bind _rootcomponent_2 (Variables|/Script/Engine.Actor|GetRootComponent _currenttarget))
  (bind _returnvalue_3 (Transformation|GetWorldTransform _rootcomponent))
  (bind _returnvalue_4 (Transformation|GetWorldTransform _rootcomponent_2))
  (bind _returnvalue_5 (Math|Rotator|FindLookatRotation (.location _returnvalue) (.location _returnvalue_3)))
  (bind _returnvalue_6 (Math|Rotator|FindLookatRotation (.location _returnvalue) (.location _returnvalue_4)))
  (bind _returnvalue_7 (- (.yaw _returnvalue_5) (.yaw (.rotation _returnvalue_2))))
  (bind _returnvalue_8 (- (.yaw _returnvalue_6) (.yaw (.rotation _returnvalue_2))))
  (bind _returnvalue_9 (+ _returnvalue_7 _returnvalue_8))
  ;[1 1 1] Define what enemys are right and what are left of the Player (Mouse Wheel Up/Down)
  (if (Math|Float|InRange(Float) (Math|Float|SelectFloat (+ _returnvalue_9 3.6e+02) _returnvalue_9 (< _returnvalue_9 0.0)) 2.4e+02 3.6e+02)
    (CallFunction|CheckDistance)))

(event Custom|EnemyToRight
  (bind _cameraboom (Variables|Default|GetCameraBoom))
  (bind _enemyelement (Variables|Default|GetEnemyElement))
  (bind _currenttarget (Variables|Default|GetCurrentTarget))
  (bind _followcamera (Variables|Default|GetFollowCamera))
  (bind _returnvalue (Transformation|GetWorldTransform _cameraboom))
  (bind _returnvalue_2 (Transformation|GetWorldTransform _followcamera))
  (bind _rootcomponent (Variables|/Script/Engine.Actor|GetRootComponent _enemyelement))
  (bind _rootcomponent_2 (Variables|/Script/Engine.Actor|GetRootComponent _currenttarget))
  (bind _returnvalue_3 (Transformation|GetWorldTransform _rootcomponent))
  (bind _returnvalue_4 (Transformation|GetWorldTransform _rootcomponent_2))
  (bind _returnvalue_5 (Math|Rotator|FindLookatRotation (.location _returnvalue) (.location _returnvalue_3)))
  (bind _returnvalue_6 (Math|Rotator|FindLookatRotation (.location _returnvalue) (.location _returnvalue_4)))
  (bind _returnvalue_7 (- (.yaw _returnvalue_5) (.yaw (.rotation _returnvalue_2))))
  (bind _returnvalue_8 (- (.yaw _returnvalue_6) (.yaw (.rotation _returnvalue_2))))
  (bind _returnvalue_9 (+ _returnvalue_7 _returnvalue_8))
  ;[1 1 1] Define what enemys are right and what are left of the Player (Mouse Wheel Up/Down)
  (if (Math|Float|InRange(Float) (Math|Float|SelectFloat (+ _returnvalue_9 3.6e+02) _returnvalue_9 (< _returnvalue_9 0.0)) 0.0 1.2e+02)
    (CallFunction|CheckDistance)))

(event Custom|Turn%20Player%20To%20Enemy
  (bind _returnvalue (Components|GetOwner))
  (bind _nearesttarget (Variables|Default|GetNearestTarget))
  (bind _asmain_character_bp (Utilities|Casting|CastToMainCharacter_BP _returnvalue))
  (bind (_rotation _isequal_) (Default|CalculatePlayerRotationtoEnemy _asmain_character_bp _nearesttarget))
  ;[1 1 1] Rotate Player to Enemy
  (if (Variables|Default|GetTargetLocked)
    (Utilities|IsValid _nearesttarget :!label _label
      (:Is%20Valid
        (if (not _isequal_)
          (Transformation|SetActorRotation (Components|GetOwner) _rotation)
          (Utilities|FlowControl|Delay 0.0)
          (goto _label))))))

(event Custom|TargetLock
  (bind _followcamera (Variables|Default|GetFollowCamera))
  (bind _returnvalue (Transformation|GetWorldLocation _followcamera))
  ;[1 1 1] Target Lock
  (Variables|Default|SetOffCenter 1.8e+02)
  (Variables|Default|SetStartVector (Math|Vector|MakeVector (.x _returnvalue) (.y _returnvalue) (+ (.z _returnvalue) 2e+02)))
  (Variables|Default|SetClosesTargetDistance (Variables|Default|GetMinimumDistanceToEnable))
  (if (Variables|Default|GetTargetLocked)
    (Variables|Default|SetTargetLocked false)
    (bind _nearesttarget (Variables|Default|GetNearestTarget :!label _label)
      (:then
        (Class|CombatBPI|TargetLockON(Message) _nearesttarget)
        (Utilities|FlowControl|Gate true) ; enters at Toggle
      )
      (:else
        (Utilities|FlowControl|Gate true) ; enters at Toggle
      ))
    (else
      (bind _outactors (Actor|GetAllActorsOfClass "/Game/Blueprints/Characters/Enemies/Enemy_ParentBP.Enemy_ParentBP_C"))
      (for _array_element _outactors
        (Variables|Default|SetEnemyElement _array_element)
        (bind _outhit (Collision|LineTraceForObjects (Transformation|GetActorLocation (Components|GetOwner)) (Transformation|GetActorLocation (Variables|Default|GetEnemyElement)) (Utilities|Array|MakeArray "ObjectTypeQuery3") false 0 "None"))
        (if (== (Variables|Default|GetEnemyElement) (.HitActor (Collision|BreakHitResult _outhit)))
          (bind _distancefromplayer (Default|DistancefromPlayerCheck (Variables|Default|GetEnemyElement)))
          (Math|Float|CompareFloat _distancefromplayer (Variables|Default|GetMinimumDistanceToEnable)
            (:<
              (CallFunction|AngleCheck)
              (Utilities|FlowControl|DoOnce false
                (:Completed
                  (CallFunction|LockOff)))))))
      (if (< (Variables|Default|GetClosesTargetDistance) (Variables|Default|GetMinimumDistanceToEnable))
        (Variables|Default|SetTargetLocked true)
        (goto _label)))))

(event Custom|AngleCheck
  (bind _cameraboom (Variables|Default|GetCameraBoom))
  (bind _enemyelement (Variables|Default|GetEnemyElement))
  (bind _followcamera (Variables|Default|GetFollowCamera))
  (bind _cameraboom_2 (Variables|Default|GetCameraBoom))
  (bind _enemyelement_2 (Variables|Default|GetEnemyElement))
  (bind _followcamera_2 (Variables|Default|GetFollowCamera))
  (bind _returnvalue (Transformation|GetWorldTransform _followcamera))
  (bind _returnvalue_2 (Transformation|GetWorldTransform _cameraboom))
  (bind _returnvalue_3 (Transformation|GetWorldTransform _cameraboom_2))
  (bind _returnvalue_4 (Transformation|GetWorldTransform _followcamera_2))
  (bind _rootcomponent (Variables|/Script/Engine.Actor|GetRootComponent _enemyelement))
  (bind _rootcomponent_2 (Variables|/Script/Engine.Actor|GetRootComponent _enemyelement_2))
  (bind _returnvalue_5 (Transformation|GetWorldTransform _rootcomponent))
  (bind _returnvalue_6 (Transformation|GetWorldTransform _rootcomponent_2))
  (bind _returnvalue_7 (Math|Rotator|FindLookatRotation (.location _returnvalue_2) (.location _returnvalue_5)))
  (bind _returnvalue_8 (Math|Rotator|FindLookatRotation (.location _returnvalue_3) (.location _returnvalue_6)))
  (bind _returnvalue_9 (- (.pitch _returnvalue_7) (.pitch (.rotation _returnvalue))))
  (bind _returnvalue_10 (- (.yaw _returnvalue_8) (.yaw (.rotation _returnvalue_4))))
  (bind _returnvalue_11 (< _returnvalue_9 0.0))
  (bind _returnvalue_12 (< _returnvalue_10 0.0))
  (bind _returnvalue_13 (+ _returnvalue_9 3.6e+02))
  (bind _returnvalue_14 (+ _returnvalue_10 3.6e+02))
  (bind _returnvalue_15 (Math|Float|SelectFloat _returnvalue_13 _returnvalue_9 _returnvalue_11))
  (bind _returnvalue_16 (Math|Float|SelectFloat _returnvalue_14 _returnvalue_10 _returnvalue_12))
  ;[1 1 1] Check Enemy that is Closest to Screen Center (in 360° Angle)
  (bind _output_get (Variables|Default|SetEnemyAngle _returnvalue_16))
  (Math|Float|CompareFloat (+ (Math|Float|SelectFloat (- 3.6e+02 _output_get) _output_get (Math|Float|InRange(Float) _returnvalue_16 2.7e+02 3.6e+02)) (* (Math|Float|NormalizetoRange (Transformation|GetDistanceTo (Components|GetOwner) (Variables|Default|GetEnemyElement)) 0.0 1e+03) (Math|Float|SelectFloat (- _returnvalue_15 3.6e+02) _returnvalue_15 (> _returnvalue_15 1.8e+02)))) (Variables|Default|GetOffCenter)
    (:==
      _)
    (:<
      _))
  (Variables|Default|SetOffCenter (+ (Math|Float|SelectFloat (- 3.6e+02 _output_get) _output_get (Math|Float|InRange(Float) _returnvalue_16 2.7e+02 3.6e+02)) (* (Math|Float|NormalizetoRange (Transformation|GetDistanceTo (Components|GetOwner) (Variables|Default|GetEnemyElement)) 0.0 1e+03) (Math|Float|SelectFloat (- _returnvalue_15 3.6e+02) _returnvalue_15 (> _returnvalue_15 1.8e+02)))))
  (bind _output_get_2 (Variables|Default|SetNearestTarget (Variables|Default|GetEnemyElement)))
  (Variables|Default|SetClosesTargetDistance (Transformation|GetDistanceTo (Components|GetOwner) _output_get_2)))

(event Custom|CheckDistance
  (bind _currenttarget (Variables|Default|GetCurrentTarget))
  (bind _enemyelement (Variables|Default|GetEnemyElement))
  (bind _returnvalue (Transformation|GetDistanceTo _currenttarget _enemyelement))
  ;[1 1 1] Check distance
  (if (< (Transformation|GetDistanceTo (Components|GetOwner) (Variables|Default|GetEnemyElement)) (Variables|Default|GetMinimumDistanceToEnable))
    (Math|Float|CompareFloat _returnvalue (Variables|Default|GetClosesTargetDistance)
      (:<
        (Variables|Default|SetClosesTargetDistance _returnvalue)
        (Variables|Default|SetNearestTarget (Variables|Default|GetEnemyElement))))))

(event EventTick
  (params (DeltaSeconds :type Float%20%28single-precision%29))
  ;[1 1 1] Target Lock
  (CallFunction|BreakLineOfSight)
  (CallFunction|DistanceLockOff)
  (Utilities|FlowControl|Gate true
    (:Exit
      (bind _nearesttarget (Variables|Default|GetNearestTarget)
        (:then
          (Pawn|SetControlRotation (.Controller (Default|CalculateCameraRotationAroundTarget (.AsMain%20Character%20BP (Utilities|Casting|CastToMainCharacter_BP (Components|GetOwner))) _nearesttarget)) (.NewRotation (Default|CalculateCameraRotationAroundTarget (.AsMain%20Character%20BP (Utilities|Casting|CastToMainCharacter_BP (Components|GetOwner))) _nearesttarget))))
        (:else)))))

(event EventBeginPlay
  ;[1 1 1] Lock Off when Player dies
  (EventDispatchers|BindEventtoDeath (Variables|/Game/Blueprints/Characters/BP_GameCharacter.BP_GameCharacter_C|GetCombatComponent (Variables|Default|GetPlayerRef)) (delegate Custom|PlayerDiesLockOff))
  (CallFunction|LockOff))