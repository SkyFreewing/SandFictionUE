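; Character stat component, marked old and not yet implemented in characters or enemies, that handles incoming weapon damage and health.
; ReceiveDamage reduces weapon damage by Armor as a percentage, subtracts it from current health, then calls Kill when health percentage nears zero.
; Kill and CheckHit are empty stubs.
; A sphere-trace helper gathers Characters within weapon range, but its only event-graph call is disconnected.
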(event Custom|ReceiveDamage
  (params (Weapon%20Stats :type Weapon%20Stats%20Structure) (Damage%20Cause :type Actor%20Object%20Reference))
  ;[1 1 1] ToDo - not implemented yet in Character or Enemies
  (bind _new_health_percentage (CallFunction|ApplyDamage (CallFunction|CalculateActualDamage Weapon%20Stats)))
  (if (Math|Float|NearlyEqual(Float) _new_health_percentage 0.0 0.01)
    (CallFunction|Kill)))

(event Custom|Check%20Hit)

(event Custom|Kill)

(fn CalculateActualDamage
  (params (Weapon%20Stats :type Weapon%20Stats%20Structure%20%28by%20ref%29))
  (bind _damage (Utilities|Struct|BreakWeaponStats Weapon%20Stats))
  (return (- _damage (* (/ _damage 1e+02) (.Armor (Utilities|Struct|BreakCharacterStat_Struct (Variables|Default|GetCharacterStats)))))))

(fn ApplyDamage
  (params (Damage :type Float%20%28single-precision%29))
  (bind _self self)
  (bind (_new_health_percentage _new_current_health) (Utilities|SetCurrentHealth _self (- (Utilities|GetCurrentHealth _self) Damage))
    (:Out
      (return _new_health_percentage _new_current_health))))

(fn CheckEnemiesinRange
  (params (WeaponHitLocation :type Vector) (WeaponRange :type Float%20%28single-precision%29) (ObjectTypes :type Array%20of%20EObjectTypeQuery%20Enums :default "ObjectTypeQuery1"))
  (bind _outhits (Collision|MultiSphereTraceForObjects WeaponHitLocation (+ WeaponHitLocation "0, 0,0.010000") WeaponRange ObjectTypes false 0 "None"))
  (for _array_element _outhits
    (bind _ascharacter (Utilities|Casting|CastToCharacter (.HitActor (Collision|BreakHitResult _array_element))))
    (Utilities|Array|Add (LocalVariables|GetActorsInRange) _ascharacter))
  (return (LocalVariables|GetActorsInRange)))