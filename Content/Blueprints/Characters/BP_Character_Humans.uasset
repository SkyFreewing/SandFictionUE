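; Human character Blueprint containing eye-blink logic that drives morph targets on the mesh.
; A RandomBlink timeline update passes through a DoOnce, plays BlinkAnim from the start, then resets after a random delay of a few seconds.
; BlinkAnim feeds its value to both eyelid morph targets through the anim instance.
; Nothing in the graph starts RandomBlink, and the construction script only calls its parent.
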(fn ConstructionScript
  (|CallParentFunction))