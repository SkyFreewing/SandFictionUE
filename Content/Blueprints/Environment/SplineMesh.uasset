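; Spline-driven environment actor that builds a chain of deformed, collidable meshes along an editable spline, entirely in the Construction Script.
; With AlignToGround enabled, it first snaps each spline point to traced ground using a vertical Visibility trace.
; It then divides the spline length by Spacing and adds a spline mesh component per segment, using world-space positions and tangents, with Offset extending each segment's end.
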(event EventBeginPlay)

(event Collision|EventActorBeginOverlap
  (params (OtherActor :type Actor%20Object%20Reference)))

(event EventTick
  (params (DeltaSeconds :type Float%20%28single-precision%29)))

(fn ConstructionScript
  (bind _spline (Variables|Default|GetSpline))
  (bind _spline_2 (Variables|Default|GetSpline))
  (bind _spacing (Variables|Default|GetSpacing))
  (if (Variables|Default|GetAlignToGround)
    (for _index (range 0 (Spline|GetNumberOfSplinePoints (Variables|Default|GetSpline)))
      (bind _outhit (Collision|LineTraceByChannel (+ (Spline|GetLocationatSplinePoint (Variables|Default|GetSpline) _index "World") "0, 0,500.000000") (- (Spline|GetLocationatSplinePoint (Variables|Default|GetSpline) _index "World") "0, 0,500.000000") "TraceTypeQuery1" true 0 "None"))
      (Spline|SetLocationatSplinePoint (Variables|Default|GetSpline) _index (.location _outhit) "World" true)))
  (for _index_2 (range 0 (- (.ReturnValue (Math|Float|Division(WholeandRemainder) (Spline|GetSplineLength (Variables|Default|GetSpline)) (Variables|Default|GetSpacing))) 1))
    (bind _returnvalue (AddComponent|AddSplineMeshComponent true))
    (Components|StaticMesh|SetStaticMesh _returnvalue (Variables|Default|GetSplineMesh))
    (SplineMesh|SetStartandEnd _returnvalue (Spline|GetLocationatDistanceAlongSpline _spline_2 (* _index_2 _spacing) "World") (Spline|GetTangentatDistanceAlongSpline _spline_2 (* _index_2 _spacing) "World") (Spline|GetLocationatDistanceAlongSpline _spline (+ (* _index_2 _spacing) _spacing (Variables|Default|GetOffset)) "World") (Spline|GetTangentatDistanceAlongSpline _spline (+ (* _index_2 _spacing) _spacing (Variables|Default|GetOffset)) "World") true :!class /Script/Engine.SplineMeshComponent)
    (Collision|SetCollisionEnabled _returnvalue "QueryAndPhysics")))