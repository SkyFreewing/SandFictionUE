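; BP_Interactable_StaticActor is a child interactable Blueprint that represents an interactable using a static mesh.
; It extends the parent's SetupMesh event, then applies its mesh, offset and scale variables to the InteractionMesh component.
; The construction script only calls the parent, and BeginPlay, overlap and Tick are disabled stubs, so all other behavior is inherited.
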(event EventBeginPlay
  (|CallParentFunction) ; This node is disabled and will not be called.\nDrag off pins to build functionality.
)

(event Collision|EventActorBeginOverlap
  (params (OtherActor :type Actor%20Object%20Reference)))

(event EventTick
  (params (DeltaSeconds :type Float%20%28single-precision%29)))

(event EventSetupMesh
  (|CallParentFunction)
  (Components|StaticMesh|SetStaticMesh (Variables|Default|GetInteractionMesh) (Variables|Mesh|GetActorMesh))
  (Transformation|SetRelativeLocation (Variables|Default|GetInteractionMesh) (Variables|Mesh|GetMeshOffset) false false)
  (Transformation|SetRelativeScale3D (Variables|Default|GetInteractionMesh) (Variables|Mesh|GetMeshScale)))

(fn ConstructionScript
  (|CallParentFunction))