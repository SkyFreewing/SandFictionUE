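; Base Blueprint for interactable pickup items that go into the player's inventory, with a UseItem function that returns true.
; The construction script fills ItemStructure from its data table row and sets the UI description from its name.
; Interact adds one item to the inventory, then plays a pickup montage and destroys the actor on success.
; While interactable, Tick toggles the highlight by player distance, using two DoOnce gates that reset each other.
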(event EventTick
  (params (DeltaSeconds :type Float%20%28single-precision%29))
  (bind _itemhighlight (Variables|Default|GetItemHighlight))
  (if (Variables|Default|GetIsInteractable)
    (if (< (Transformation|GetDistanceTo (Game|GetPlayerCharacter 0)) (Variables|Default|GetHighlightRange))
      (Utilities|FlowControl|DoOnce false :!label _label
        (:Completed
          (Components|Activation|Activate _itemhighlight false)
          (Rendering|SetVisibility _itemhighlight true false)
          (goto _label_2 Reset)))
      (else
        (Utilities|FlowControl|DoOnce false :!label _label_2
          (:Completed
            (Components|Activation|Deactivate _itemhighlight)
            (Rendering|SetVisibility _itemhighlight false false)
            (goto _label Reset)))))))

(event EventInteract
  (params (Player :type Main%20Character%20BP%20Object%20Reference))
  (|CallParentFunction Player)
  (bind _success (Default|AddtoInventory (Variables|/Game/Blueprints/Characters/MainCharacter/MainCharacter_BP.MainCharacter_BP_C|GetInventory Player) (Utilities|Struct|MakeInventorySlotStructure (Variables|Default|GetItemStructure) 1) false))
  (if _success
    (Animation|Montage|MontagePlay (Components|SkeletalMesh|GetAnimInstance (Variables|/Script/Engine.Character|GetMesh (Variables|Default|GetPlayer))) "/Game/Blueprints/Characters/MainCharacter/Animations/MainCharacter_PickUpAnimMontage.MainCharacter_PickUpAnimMontage" 1.0 "MontageLength" 0.0 true)
    (Actor|DestroyActor)
    (else
      (Development|PrintString "NotAdded"))))

(fn ConstructionScript
  (bind _returnvalue (Utilities|GetDataTableRow (.datatable (.datatableitem (Variables|Default|GetItemStructure))) (.rowname (.datatableitem (Variables|Default|GetItemStructure))))
    (:then
      (Variables|Default|SetItemStructure _returnvalue))
    (:RowNotFound
      _))
  (Variables|Default|SetUIDescription (.name (Variables|Default|GetItemStructure)))
  (|CallParentFunction))

(fn UseItem
  (return true))