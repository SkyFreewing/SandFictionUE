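; Volume that scatters material nodes within a sphere radius and refills them to a target count at each midnight from BP_TimeOfDay.
; On begin play and midnight it spawns randomly scaled nodes at random navigable points, after pruning invalid entries on midnight refills.
; A line trace snaps each node to the surface with a Z offset and aligns it to the normal.
; The construction script sizes the sphere and sets the billboard to the item's data table icon.
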(event Custom|SpawnMaterialNodes
  (CallFunction|UpdateItemArray)
  (CallFunction|RespawnNodes))

(event EventBeginPlay
  (CallFunction|RespawnNodes)
  (bind _returnvalue (Actor|GetActorOfClass "/Game/Blueprints/BP_TimeOfDay.BP_TimeOfDay_C"))
  (bind _output_get (Variables|Default|SetBPTimeOfDay _returnvalue))
  (EventDispatchers|BindEventtoMidNight _output_get (delegate Custom|SpawnMaterialNodes)))

(fn ConstructionScript
  (bind _materialnodetospawn (Variables|Default|GetMaterialNodeToSpawn))
  (bind _itemstructure (Utilities|GetClassDefaults _materialnodetospawn))
  (Components|Sphere|SetSphereRadius (Variables|Default|GetSpawnVolume) (Variables|Default|GetSphereRadius) true)
  (bind _returnvalue (Utilities|GetDataTableRow (.datatable (.datatableitem _itemstructure)) (.rowname (.datatableitem _itemstructure)))
    (:then
      (Rendering|Components|Sprite|SetSprite (Variables|Default|GetBillboard) (.Icon (Utilities|Struct|BreakItemStructure _returnvalue))))))

(fn RespawnNodes
  (bind _minsize (Variables|Default|GetMinSize))
  (bind _maxsize (Variables|Default|GetMaxSize))
  (bind _returnvalue (Math|Random|RandomFloatinRange _minsize _maxsize))
  (while (!= (Utilities|Array|Length (Variables|Default|GetSpawnedMaterialNodes)) (Variables|Default|GetNumberOfNodesToSpawn))
    (bind _returnvalue_2 (Game|SpawnActorfromClass (Variables|Default|GetMaterialNodeToSpawn) (Math|Transform|MakeTransform (.RandomLocation (Class|NavigationSystemV1|GetRandomPointinNavigableRadius (Transformation|GetActorLocation) (Variables|/Script/Engine.SphereComponent|GetSphereRadius (Variables|Default|GetSpawnVolume)) 0 0)) (Math|Rotator|MakeRotator 0.0 0.0 (Math|Random|RandomFloatinRange -1.8e+02 1.8e+02)) (Math|Vector|MakeVector _returnvalue _returnvalue _returnvalue)) "Undefined" 0 true true 0))
    (Utilities|Array|Add (Variables|Default|GetSpawnedMaterialNodes) _returnvalue_2)
    (bind _outhit (Collision|LineTraceByChannel (+ (Transformation|GetActorLocation _returnvalue_2) "0, 0,200.000000") (- (Transformation|GetActorLocation _returnvalue_2) "0, 0,200.000000") "TraceTypeQuery1" true (Variables|Default|GetSpawnedMaterialNodes) "None"))
    (Transformation|SetActorLocationAndRotation _returnvalue_2 (+ (.location _outhit) (Math|Vector|MakeVector 0.0 0.0 (Variables|Default|GetZOffset))) (Math|Rotator|MakeRotfromZ (.normal _outhit))))
  (Development|PrintString (Utilities|String|ToString(Integer) (Utilities|Array|Length (Variables|Default|GetSpawnedMaterialNodes)))))

(fn UpdateItemArray
  (for _array_element (Variables|Default|GetSpawnedMaterialNodes)
    (Utilities|IsValid _array_element
      (:Is%20Valid
        (Utilities|Array|Add (LocalVariables|GetNewSpawnedMaterialNodesArray) _array_element))))
  (Variables|Default|SetSpawnedMaterialNodes (LocalVariables|GetNewSpawnedMaterialNodesArray))
  (return))