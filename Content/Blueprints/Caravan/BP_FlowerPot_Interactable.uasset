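; Caravan flower pot interactable that grows a planted seed into a plant over seven in-game days.
; AddSeed starts growth and shows the first stage, and a BP_TimeOfDay day-time event advances a counter that switches stage meshes at thresholds until the PlantActor child actor appears.
; Interact only casts that child to Item_Parent, behind a full-growth check the counter never satisfies because it resets on completion.
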(event Custom|Grow
  (if (Variables|Default|GetIsGrowing)
    (bind _result (Math|Integer|IncrementInt (Variables|Default|GetCurrentGrowth))
      (:%20%20
        (if (== _result 1)
          (Rendering|SetVisibility (Variables|Default|GetFlowerPot_Stage02) true false)
          (elif (== _result 4)
            (Rendering|SetVisibility (Variables|Default|GetFlowerPot_Stage03) true false)
            (Rendering|SetVisibility (Variables|Default|GetFlowerPot_Stage02) false false)
            (elif (== _result 7)
              (Rendering|SetVisibility (Variables|Default|GetPlantActor) true false)
              (Rendering|SetVisibility (Variables|Default|GetFlowerPot_Stage03) false false)
              (Rendering|SetVisibility (Variables|Default|GetFlowerPot_Stage02) false false)
              (Variables|Default|SetIsGrowing false)
              (Variables|Default|SetCurrentGrowth 0))))))))

(event Custom|AddSeed
  (Variables|Default|SetIsGrowing true)
  (Variables|Default|SetCurrentGrowth 0)
  (Rendering|SetVisibility (Variables|Default|GetFlowerPot_Stage01) true false))

(event EventBeginPlay
  (bind _returnvalue (Actor|GetActorOfClass "/Game/Blueprints/BP_TimeOfDay.BP_TimeOfDay_C"))
  (EventDispatchers|BindEventtoDayTime _returnvalue (delegate Custom|Grow)))

(event EventInteract
  (params (Player :type Main%20Character%20BP%20Object%20Reference))
  (if (== (Variables|Default|GetCurrentGrowth) 7)
    (Utilities|Casting|CastToItem_Parent (Variables|/Script/Engine.ChildActorComponent|GetChildActor (Variables|Default|GetPlantActor)))))

(fn ConstructionScript)