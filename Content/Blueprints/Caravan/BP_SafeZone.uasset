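; BP_SafeZone is a caravan safe-zone volume that tracks whether the main character is inside it.
; The construction script sizes its SafeZone sphere component from the CaravanRadius variable.
; Actor begin and end overlap events cast to MainCharacter_BP, set its IsInSafeZone flag true or false, and print a debug message.
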(event Collision|EventActorBeginOverlap
  (params (OtherActor :type Actor%20Object%20Reference))
  (bind _asmain_character_bp (Utilities|Casting|CastToMainCharacter_BP OtherActor))
  (Variables|/Game/Blueprints/Characters/MainCharacter/MainCharacter_BP.MainCharacter_BP_C|SetIsInSafeZone _asmain_character_bp true)
  (Development|PrintString "Player Entered SafeZone"))

(event Collision|EventActorEndOverlap
  (params (OtherActor :type Actor%20Object%20Reference))
  (bind _asmain_character_bp (Utilities|Casting|CastToMainCharacter_BP OtherActor))
  (Variables|/Game/Blueprints/Characters/MainCharacter/MainCharacter_BP.MainCharacter_BP_C|SetIsInSafeZone _asmain_character_bp false)
  (Development|PrintString "Player Leaves SafeZone"))

(fn ConstructionScript
  (Components|Sphere|SetSphereRadius (Variables|Default|GetSafeZone) (Variables|Default|GetCaravanRadius) true))