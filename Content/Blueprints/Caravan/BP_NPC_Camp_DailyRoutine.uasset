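; Placeable daily-routine point for a camp NPC, which triggers at a set time of day.
; BeginPlay finds the time-of-day actor and an NPC of the configured class.
; Tick compares StartTime to the current time and, if the NPC's blackboard enables routines, writes itself as DailyRoutineActor, with a delayed DoOnce reset limiting retriggers.
; The construction script labels it with class and hour; a direct AIMoveTo chain is left unconnected.
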(event Custom|Do%20Behavior
  (Development|PrintString (Utilities|String|ToString(Text) (Utilities|Text|FormatText "{NPC} started Daily Routine" (Variables|/Game/Blueprints/Characters/NPCs/NPC_Parent.NPC_Parent_C|GetName (Variables|Default|GetNPC)))))
  (AI|Components|Blackboard|SetValueasObject (AI|GetBlackboard (Variables|Default|GetNPC)) (Utilities|Name|MakeLiteralName "DailyRoutineActor") self))

(event EventBeginPlay
  (bind _returnvalue (Actor|GetActorOfClass "/Game/Blueprints/BP_TimeOfDay.BP_TimeOfDay_C"))
  (Variables|Default|SetTimeRef _returnvalue)
  (bind _returnvalue_2 (Actor|GetActorOfClass (Variables|Default|GetNPC%20Class)))
  (Variables|Default|SetNPC _returnvalue_2)
  (Actor|Tick|SetActorTickEnabled true))

(event EventTick
  (params (DeltaSeconds :type Float%20%28single-precision%29))
  (if (and (Math|Float|NearlyEqual(Float) (Variables|Default|GetStartTime) (Variables|/Game/Blueprints/BP_TimeOfDay.BP_TimeOfDay_C|GetCurrentTime (Variables|Default|GetTimeRef)) 0.1) (ScalableFloat|GetValueasBool (AI|GetBlackboard (Variables|Default|GetNPC)) (Utilities|Name|MakeLiteralName "DailyRoutineEnabled")))
    (Utilities|FlowControl|DoOnce false :!label _label
      (:Completed
        (CallFunction|DoBehavior)
        (Utilities|FlowControl|Delay 1e+01)
        (goto _label Reset)))))

(fn ConstructionScript
  (Rendering|Components|TextRender|SetText (Variables|Default|GetTextRender) (Utilities|Text|FormatText "{Name} 
{Time}:00" (Utilities|GetClassDefaults (Variables|Default|GetNPC%20Class)) (Math|Float|Floor (Variables|Default|GetStartTime)))))