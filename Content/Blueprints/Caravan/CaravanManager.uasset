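; Caravan manager that shows or removes the caravan's blacksmith, cooking, clothing and woodworking stations according to one boolean per station.
; BeginPlay caches the transforms of the referenced station actors, then calls UpdateCaravanStatus.
; That event spawns any enabled but missing station at its cached transform, storing the new reference, and destroys any disabled station that still exists.
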(event Custom|Update%20Caravan%20Status
  (Development|PrintString "Caravan Updated")
  (Utilities|FlowControl|Sequence
    (:then_0
      (if (Variables|Default|GetBlacksmithStation)
        (Variables|Default|GetBlacksmithActor
          (:then)
          (:else
            (bind _returnvalue (Game|SpawnActorfromClass "/Game/Blueprints/Caravan/BP_BlacksmithsStation.BP_BlacksmithsStation_C" (Variables|Default|GetBlacksmithTransform) "AlwaysSpawn" 0 0))
            (Variables|Default|SetBlacksmithActor _returnvalue)))
        (else
          (bind _blacksmithactor (Variables|Default|GetBlacksmithActor)
            (:then
              (Actor|DestroyActor _blacksmithactor))
            (:else)))))
    (:then_1
      (if (Variables|Default|GetCookingStation)
        (Variables|Default|GetCookingActor
          (:then)
          (:else
            (bind _returnvalue_2 (Game|SpawnActorfromClass "/Game/Blueprints/Caravan/BP_Campfire.BP_Campfire_C" (Variables|Default|GetCookingTransform) "AlwaysSpawn" 0 0))
            (Variables|Default|SetCookingActor _returnvalue_2)))
        (else
          (bind _cookingactor (Variables|Default|GetCookingActor)
            (:then
              (Actor|DestroyActor _cookingactor))
            (:else)))))
    (:then_2
      (if (Variables|Default|GetClothingStation)
        (Variables|Default|GetClothingActor
          (:then)
          (:else
            (bind _returnvalue_3 (Game|SpawnActorfromClass "/Game/Blueprints/Caravan/InayaCart_Blueprint.InayaCart_Blueprint_C" (Variables|Default|GetClothingTransform) "AlwaysSpawn" 0 0))
            (Variables|Default|SetClothingActor _returnvalue_3)))
        (else
          (bind _clothingactor (Variables|Default|GetClothingActor)
            (:then
              (Actor|DestroyActor _clothingactor))
            (:else)))))
    (:then_3
      (if (Variables|Default|GetWoodworkingStation)
        (Variables|Default|GetWoodworkingActor
          (:then)
          (:else
            (bind _returnvalue_4 (Game|SpawnActorfromClass "/Game/Blueprints/Caravan/BP_InventorsBench.BP_InventorsBench_C" (Variables|Default|GetWoodworkingTransform) "AlwaysSpawn" 0 0))
            (Variables|Default|SetWoodworkingActor _returnvalue_4)))
        (else
          (bind _woodworkingactor (Variables|Default|GetWoodworkingActor)
            (:then
              (Actor|DestroyActor _woodworkingactor))
            (:else)))))))

(event EventBeginPlay
  (Variables|Default|SetBlacksmithTransform (Transformation|GetActorTransform (Variables|Default|GetBlacksmithActor)))
  (Variables|Default|SetCookingTransform (Transformation|GetActorTransform (Variables|Default|GetCookingActor)))
  (Variables|Default|SetClothingTransform (Transformation|GetActorTransform (Variables|Default|GetClothingActor)))
  (Variables|Default|SetWoodworkingTransform (Transformation|GetActorTransform (Variables|Default|GetWoodworkingActor)))
  (CallFunction|UpdateCaravanStatus))

(fn ConstructionScript)