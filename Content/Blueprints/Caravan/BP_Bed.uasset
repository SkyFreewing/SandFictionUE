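; BP_Bed is an interactable bed in the Caravan set that lets the player sleep to change the time of day and heal.
; On BeginPlay it caches the level's BP_TimeOfDay actor.
; Interact plays the sleep montage on the player's mesh, then calls ChangeTime on that actor and Heal on the player's CombatComponent right away, without waiting for the montage to finish.
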(event EventBeginPlay
  (|CallParentFunction)
  (bind _returnvalue (Actor|GetActorOfClass "/Game/Blueprints/BP_TimeOfDay.BP_TimeOfDay_C"))
  (Variables|Default|SetTimeOfDay _returnvalue))

(event EventInteract
  (params (Player :type Main%20Character%20BP%20Object%20Reference))
  (|CallParentFunction Player)
  (Animation|Montage|PlayMontage (Variables|/Script/Engine.Character|GetMesh Player) "/Game/Blueprints/Characters/MainCharacter/Animations/Misc/MainChar_sleep.MainChar_sleep" 0.8
    (:then
      (Default|ChangeTime (Variables|Default|GetTimeOfDay) 8.0)
      (Default|Heal (Variables|/Game/Blueprints/Characters/BP_GameCharacter.BP_GameCharacter_C|GetCombatComponent Player) 1e+02 1.0))))

(fn ConstructionScript
  (|CallParentFunction))