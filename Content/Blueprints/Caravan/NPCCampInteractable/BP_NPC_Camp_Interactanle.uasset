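; Scheduled camp spot that sends an NPC of a set class to this actor at a given time of day to play a montage.
; Tick compares BP_TimeOfDay against StartTime, skipping NPCs that are following or in dialogue.
; The NPC walks over non-interactable at reduced speed, then a timeline aligns it to the actor before the montage.
; The construction script labels the spot with NPC name and hour.
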(event Custom|Do%20Behavior
  (bind _npc (Variables|Default|GetNPC))
  (bind _npc_2 (Variables|Default|GetNPC))
  (bind _charactermovement (Variables|/Script/Engine.Character|GetCharacterMovement _npc))
  (bind _returnvalue (Animation|GetCurrentMontage _npc_2 :!class /Script/Engine.Character))
  (Animation|StopAnimMontage _npc_2 _returnvalue)
  (Variables|/Game/Blueprints/UI/Interactables/BP_Interactable_Parent_Actor.BP_Interactable_Parent_Actor_C|SetIsInteractable (Variables|/Game/Blueprints/Characters/NPCs/NPC_Parent.NPC_Parent_C|GetNPC%20Interactable _npc) false)
  (Variables|Default|SetOldWalkSpeed (Variables|/Script/Engine.CharacterMovementComponent|GetMaxWalkSpeed _charactermovement))
  (Variables|/Script/Engine.CharacterMovementComponent|SetMaxWalkSpeed _charactermovement 1.5e+02)
  (AI|AIMoveTo (AI|GetAIController _npc) "0, 0, 0" self 1e+01 "Default" "Default" true true
    (:OnMoveFinished
      (Components|Timeline|PlayfromStart (Variables|Default|GetRotateNPC))
      (Variables|/Game/Blueprints/UI/Interactables/BP_Interactable_Parent_Actor.BP_Interactable_Parent_Actor_C|SetIsInteractable (Variables|/Game/Blueprints/Characters/NPCs/NPC_Parent.NPC_Parent_C|GetNPC%20Interactable (Variables|Default|GetNPC)) true)
      (Variables|/Script/Engine.CharacterMovementComponent|SetMaxWalkSpeed (Variables|/Script/Engine.Character|GetCharacterMovement (Variables|Default|GetNPC)) (Variables|Default|GetOldWalkSpeed)))))

(event EventBeginPlay
  (bind _returnvalue (Actor|GetActorOfClass "/Game/Blueprints/BP_TimeOfDay.BP_TimeOfDay_C"))
  (Variables|Default|SetTimeRef _returnvalue)
  (Utilities|FlowControl|Delay 2.0)
  (bind _returnvalue_2 (Actor|GetActorOfClass (Variables|Default|GetNPC%20Class)))
  (Variables|Default|SetNPC _returnvalue_2)
  (Actor|Tick|SetActorTickEnabled true))

(event EventTick
  (params (DeltaSeconds :type Float%20%28single-precision%29))
  (bind _npc (Variables|Default|GetNPC))
  (Utilities|FlowControl|Delay 1.0)
  (if (Math|Boolean|ANDBoolean (Math|Float|NearlyEqual(Float) (Variables|Default|GetStartTime) (Variables|/Game/Blueprints/BP_TimeOfDay.BP_TimeOfDay_C|GetCurrentTime (Variables|Default|GetTimeRef)) 0.1) (!= (Variables|/Game/Blueprints/Characters/NPCs/NPC_Parent.NPC_Parent_C|GetBehaviorTree _npc) "/Game/Blueprints/Characters/NPCs/BehaviorTrees/NPC_Follow.NPC_Follow") (not (Utilities|IsValid (Variables|/Game/Blueprints/Characters/NPCs/NPC_Interactable.NPC_Interactable_C|GetDialogRef (Variables|/Game/Blueprints/Characters/NPCs/NPC_Parent.NPC_Parent_C|GetNPC%20Interactable _npc)))))
    (Utilities|FlowControl|DoOnce false
      (:Completed
        (CallFunction|DoBehavior)))))

(fn ConstructionScript
  (Rendering|Components|TextRender|SetText (Variables|Default|GetTextRender) (Utilities|Text|FormatText "{Name} 
{Time}:00" (Utilities|GetClassDefaults (Variables|Default|GetNPC%20Class)) (Math|Float|Floor (Variables|Default|GetStartTime)))))