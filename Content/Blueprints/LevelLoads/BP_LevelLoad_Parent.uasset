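; Parent Blueprint for an interactable level transition that swaps streamed levels and teleports the player.
; Interact plays the interaction mesh, shows a loading screen widget, then loads and unloads up to five levels from each list through sequential latent stream calls.
; It then moves the player to the new transform, removes the widget and unloads its own level with a blocking call.
; The Interior event does nothing.
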(event Custom|Load%20Levels
  (bind _levelstoload (Variables|Default|GetLevelsToLoad))
  (bind _output (Utilities|Array|Get(acopy) _levelstoload 4))
  (bind _output_2 (Utilities|Array|Get(acopy) _levelstoload))
  (bind _output_3 (Utilities|Array|Get(acopy) _levelstoload 1))
  (bind _output_4 (Utilities|Array|Get(acopy) _levelstoload 2))
  (bind _output_5 (Utilities|Array|Get(acopy) _levelstoload 3))
  (if (Utilities|Array|IsValidIndex _levelstoload)
    (Game|LoadStreamLevel(byName) _output_2 true)
    (Development|PrintString (Utilities|String|ToString(Name) _output_2))
    (if (Utilities|Array|IsValidIndex _levelstoload 1)
      (Game|LoadStreamLevel(byName) _output_3 true)
      (Development|PrintString (Utilities|String|ToString(Name) _output_3))
      (if (Utilities|Array|IsValidIndex _levelstoload 2)
        (Game|LoadStreamLevel(byName) _output_4 true)
        (Development|PrintString (Utilities|String|ToString(Name) _output_4))
        (if (Utilities|Array|IsValidIndex _levelstoload 3)
          (Game|LoadStreamLevel(byName) _output_5 true)
          (Development|PrintString (Utilities|String|ToString(Name) _output_5))
          (if (Utilities|Array|IsValidIndex _levelstoload 4)
            (Game|LoadStreamLevel(byName) _output true)
            (Development|PrintString (Utilities|String|ToString(Name) _output)))))))
  (CallFunction|UnloadLevels))

(event Custom|Remove%20Widget%20And%20Set%20Player%20Transform
  (bind _newplayertransform (Variables|Default|GetNewPlayerTransform))
  (Transformation|SetActorTransform (stale EventInteract Player) (Math|Transform|MakeTransform (.location _newplayertransform) (.rotation _newplayertransform) "1,1,1") false true)
  (Utilities|FlowControl|Delay 1.0)
  (Widget|RemovefromParent (stale EventInteract _widget))
  (CallFunction|UnloadSelf))

(event Custom|Unload%20Levels
  (bind _levelstounload (Variables|Default|GetLevelsToUnload))
  (bind _output (Utilities|Array|Get(acopy) _levelstounload))
  (bind _output_2 (Utilities|Array|Get(acopy) _levelstounload 1))
  (if (Utilities|Array|IsValidIndex _levelstounload)
    (Game|UnloadStreamLevel(byName) _output false)
    (Development|PrintString (Utilities|String|ToString(Name) _output))
    (if (Utilities|Array|IsValidIndex _levelstounload 1)
      (Game|UnloadStreamLevel(byName) _output_2 false)
      (Development|PrintString (Utilities|String|ToString(Name) _output_2))
      (if (Utilities|Array|IsValidIndex _levelstounload 2)
        (Game|UnloadStreamLevel(byName) (Utilities|Array|Get(acopy) _levelstounload 2) false)
        (if (Utilities|Array|IsValidIndex _levelstounload 3)
          (Game|UnloadStreamLevel(byName) (Utilities|Array|Get(acopy) _levelstounload 3) false)
          (if (Utilities|Array|IsValidIndex _levelstounload 4)
            (Game|UnloadStreamLevel(byName) (Utilities|Array|Get(acopy) _levelstounload 4) false))))))
  (Development|PrintString "No Level To Unload")
  (CallFunction|RemoveWidgetandSetPlayerTransform))

(event Custom|Interior
  (if (Variables|Default|GetInterior?)
    _))

(event Custom|Unload%20Self
  (Game|UnloadStreamLevel(byName) (Variables|Default|GetLevelNameSelf) true))

(event EventInteract
  (params (Player :type Main%20Character%20BP%20Object%20Reference))
  (Audio|Components|Audio|Play (Variables|Default|GetInteractionMesh) false)
  (Utilities|FlowControl|Delay 1.0)
  (bind _widget (CallFunction|CreateLoadingScreen))
  (Utilities|FlowControl|Delay 1.0)
  (CallFunction|LoadLevels))

(fn ConstructionScript
  (|CallParentFunction))

(fn CreateLoadingScreen
  (bind _returnvalue (UserInterface|CreateWidget "/Game/Blueprints/UI/LoadingscreenWidget.LoadingscreenWidget_C"))
  (UserInterface|Viewport|AddtoViewport _returnvalue 0)
  (return _returnvalue))