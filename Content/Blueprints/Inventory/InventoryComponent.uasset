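; Actor component that holds a slot-based inventory, handling item stacking, quantity queries and the inventory window.
; PrepareInventory sizes the slot array and refreshes filled slots from their item class defaults.
; AddToInventory tops up a partial stack or claims an empty slot, recursively re-adding any overflow beyond max stack size.
; ToggleInventory opens or closes the centre-anchored widget on the main character's HUD canvas, switching input mode and cursor.
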(event EventBeginPlay
  (CallFunction|PrepareInventory))

(fn ToggleInventory
  (bind _returnvalue (Game|GetPlayerController 0))
  (bind _returnvalue_2 (Game|GetPlayerController 0))
  (Variables|Default|GetInventoryWindow
    (:then
      (Widget|RemovefromParent (Variables|Default|GetInventoryWindow))
      (Variables|Default|SetInventoryWindow 0)
      (Input|SetInputModeGameOnly _returnvalue_2)
      (Variables|/Script/Engine.PlayerController|SetbShowMouseCursor _returnvalue_2 false))
    (:else
      (CallFunction|PrepareInventory)
      (bind _returnvalue_3 (UserInterface|CreateWidget "/Game/Blueprints/Inventory/InventoryWindow.InventoryWindow_C" 0 self))
      (Variables|Default|SetInventoryWindow _returnvalue_3)
      (bind _asmain_character_bp (Utilities|Casting|CastToMainCharacter_BP (Game|GetPlayerCharacter 0)))
      (bind _returnvalue_4 (Class|CanvasPanel|AddChildtoCanvas (Variables|/Game/Blueprints/Characters/MainCharacter/UI/PlayerHUDWidget.PlayerHUDWidget_C|GetHUDCanvas (Variables|/Game/Blueprints/Characters/MainCharacter/MainCharacter_BP.MainCharacter_BP_C|GetHUDReference _asmain_character_bp)) (Variables|Default|GetInventoryWindow)))
      (Class|CanvasPanelSlot|SetAutoSize _returnvalue_4 true)
      (Class|CanvasPanelSlot|SetAlignment _returnvalue_4 "(X=0.500000,Y=0.500000)")
      (Class|CanvasPanelSlot|SetAnchors _returnvalue_4 (Utilities|Struct|MakeAnchors "(X=0.500000,Y=0.500000)" "(X=0.500000,Y=0.500000)"))
      (Class|CanvasPanelSlot|SetPosition _returnvalue_4 (Variables|Default|GetPosition))
      (Input|SetInputModeUIOnly _returnvalue (Variables|Default|GetInventoryWindow) "LockAlways")
      (Variables|/Script/Engine.PlayerController|SetbShowMouseCursor _returnvalue true))))

(fn AddtoInventory
  (params (ContentToAdd :type Slot%20Structure%20Structure))
  (if (.isstackable (.itemstructure ContentToAdd))
    (bind _stackindex (Utilities|HasPartialStack ContentToAdd)
      (:True
        (CallFunction|AddtoStack ContentToAdd _stackindex)
        (LocalVariables|SetAddToInventorySuccess true))
      (:False
        (bind _success (CallFunction|CreateStack ContentToAdd :!label _label))
        (LocalVariables|SetAddToInventorySuccess _success)))
    (else
      (goto _label)))
  (return (LocalVariables|GetAddToInventorySuccess)))

(fn PrepareInventory
  (Utilities|Array|Resize (Variables|Default|GetInventory) (Variables|Default|GetNumberSlots))
  (for (_array_element _array_index) (Variables|Default|GetInventory)
    (if (!= (.Class (Utilities|Struct|BreakItemStructure (.itemstructure _array_element))) 0)
      (Utilities|Array|SetArrayElem (Variables|Default|GetInventory) _array_index (Utilities|Struct|MakeSlotStructure (Utilities|GetClassDefaults (.Class (Utilities|Struct|BreakItemStructure (.itemstructure _array_element)))) (.quantity _array_element))))))

(fn CreateStack
  (params (ContentToAdd :type Slot%20Structure%20Structure))
  (bind _slotstructure (Utilities|Struct|MakeSlotStructure "(Name_2_FCF230264C23E18A21D5EB8B6DBB70C3=NSLOCTEXT(\"[E286B2974F57BA0013AB04A483DBDF24]\", \"C7D9864D4F86D7CDEFB032911806FCD6\", \"None\"),IsStackable_5_B97B3C0040D8D0E286FCEE83A9019719=True,Icon_8_3B5E6ADD44643CA1284E0AB9627A2A1A=None,Description_11_B64901DE49608EA771710BACAF48FF62=NSLOCTEXT(\"[E286B2974F57BA0013AB04A483DBDF24]\", \"520955C54D387EF46411C89400184912\", \"None\"),IsConsumable_14_4A0D5A3E4B2AB4BAE27E2CB3258874BB=True,MaxStackSize_17_799F31B946969B6759B7E0A12AD7235D=10,Durability_20_BD6C8C1C4ECEC3237AE27BA9EF273006=0.000000,Class_23_0B9D15814604799132851ABCAA1A3674=None)"))
  (bind _inventory (Variables|Default|GetInventory))
  (bind _inventory_2 (Variables|Default|GetInventory))
  (bind _returnvalue (Utilities|Array|FindItem _inventory_2 _slotstructure))
  (if (== _returnvalue -1)
    (LocalVariables|SetCreateStackSuccess false)
    (else
      (if (> (.quantity ContentToAdd) (.maxstacksize (.itemstructure ContentToAdd)))
        (Utilities|Array|SetArrayElem _inventory _returnvalue (Utilities|Struct|MakeSlotStructure (.itemstructure ContentToAdd) (.maxstacksize (.itemstructure ContentToAdd))))
        (CallFunction|AddtoInventory (Utilities|Struct|MakeSlotStructure (.itemstructure ContentToAdd) (- (.quantity ContentToAdd) (.maxstacksize (.itemstructure ContentToAdd)))))
        (else
          (Utilities|Array|SetArrayElem _inventory _returnvalue ContentToAdd)))
      (LocalVariables|SetCreateStackSuccess true)))
  (return (LocalVariables|GetCreateStackSuccess)))

(fn AddtoStack
  (params (SlotStructure :type Slot%20Structure%20Structure) (SlotIndex :type Integer))
  (bind _inventory (Variables|Default|GetInventory))
  (bind _inventory_2 (Variables|Default|GetInventory))
  (bind _maxstacksize (Utilities|Struct|BreakItemStructure (.itemstructure SlotStructure)))
  (bind _output (Utilities|Array|Get(acopy) _inventory SlotIndex))
  (bind _output_2 (Utilities|Array|Get(acopy) _inventory_2 SlotIndex))
  (bind _output_get (LocalVariables|SetCurrentQuantity (.quantity _output)))
  (if (> (+ _output_get (.Quantity (Utilities|Struct|BreakSlotStructure SlotStructure))) (.maxstacksize (.itemstructure _output)))
    (Utilities|Array|SetArrayElem (Variables|Default|GetInventory) SlotIndex (Utilities|Struct|MakeSlotStructure (.itemstructure SlotStructure) _maxstacksize))
    (CallFunction|AddtoInventory (Utilities|Struct|MakeSlotStructure (.itemstructure SlotStructure) (- (.quantity SlotStructure) (- _maxstacksize (LocalVariables|GetCurrentQuantity)))))
    (else
      (Utilities|Array|SetArrayElem _inventory_2 SlotIndex (Utilities|Struct|MakeSlotStructure (.itemstructure _output_2) (+ (.quantity _output_2) (.quantity SlotStructure))))))
  (return))

(fn InventoryQuery
  (params (QueryItem :type Item%20Parent%20Class%20Reference) (QueryAmount :type Integer))
  (for _array_element (Variables|Default|GetInventory)
    (if (== (.Class (Utilities|Struct|BreakItemStructure (.itemstructure _array_element))) QueryItem)
      (LocalVariables|SetRunningTotal (+ (.quantity _array_element) (LocalVariables|GetRunningTotal)))))
  (return (>= (LocalVariables|GetRunningTotal) QueryAmount)))