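; Dynamic camera component that shifts a camera boom around its anchor based on where the follow camera looks relative to the owner.
; InitializeCamera supplies the camera, boom and anchor references.
; CameraLocation offsets the anchor forward by camera pitch and absolute wrapped yaw difference, plus a unit-clamped sideways term, all divided by YawIntensity.
; Tick eases the boom toward that target with VInterpTo, looping through zero-second delays until within tolerance.
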(event Custom|Initialize%20Camera
  (params (FollowCamera :type Camera%20Component%20Object%20Reference) (CameraBoom :type Spring%20Arm%20Component%20Object%20Reference) (BoomAnchor :type Static%20Mesh%20Component%20Object%20Reference))
  (Variables|Default|SetFollowCamera FollowCamera)
  (Variables|Default|SetCameraBoom CameraBoom)
  (Variables|Default|SetBoomAnchor BoomAnchor))

(event EventTick
  (params (DeltaSeconds :type Float%20%28single-precision%29))
  (Variables|Default|SetTargetLocation (CallFunction|CameraLocation))
  (if (Math|Vector|Equal(Vector) (Variables|Default|GetCurrentLocation) (Variables|Default|GetTargetLocation) 1.0) :!label _label
    (Variables|Default|SetCurrentLocation (Transformation|GetWorldLocation (Variables|Default|GetCameraBoom)))
    (else
      (bind _output_get (Variables|Default|SetCurrentLocation (Math|Interpolation|VInterpTo (Variables|Default|GetCurrentLocation) (Variables|Default|GetTargetLocation) (Utilities|Time|GetWorldDeltaSeconds) (Variables|Default|GetAdjustmentSpeed))))
      (Transformation|SetWorldLocation (Variables|Default|GetCameraBoom) _output_get false false)
      (Utilities|FlowControl|Delay 0.0)
      (goto _label))))

(fn CameraLocation
  (bind _returnvalue (Components|GetOwner))
  (bind _boomanchor (Variables|Default|GetBoomAnchor))
  (bind _followcamera (Variables|Default|GetFollowCamera))
  (bind _returnvalue_2 (Transformation|GetWorldLocation _boomanchor))
  (bind _returnvalue_3 (Math|Vector|GetForwardVector _boomanchor))
  (bind _returnvalue_4 (Transformation|GetActorRotation _returnvalue))
  (bind _returnvalue_5 (Transformation|GetWorldRotation _followcamera))
  (bind _returnvalue_6 (- (.yaw _returnvalue_4) (.yaw _returnvalue_5)))
  (bind _returnvalue_7 (< _returnvalue_6 0.0))
  (bind _returnvalue_8 (+ _returnvalue_6 3.6e+02))
  (bind _returnvalue_9 (Math|Float|SelectFloat _returnvalue_8 _returnvalue_6 _returnvalue_7))
  (bind _returnvalue_10 (- _returnvalue_9 3.6e+02))
  (bind _returnvalue_11 (< 1.8e+02 _returnvalue_9))
  (bind _returnvalue_12 (Math|Float|SelectFloat _returnvalue_10 _returnvalue_9 _returnvalue_11))
  (return (+ _returnvalue_2 (/ (- (+ _returnvalue_2 (+ (* _returnvalue_3 (* (* (.pitch (.rotation (Transformation|GetWorldTransform (Variables|Default|GetFollowCamera)))) -1.0) (Variables|Default|GetPitchIntensity))) (+ (* _returnvalue_3 (Math|Float|SelectFloat (* _returnvalue_12 -1.0) _returnvalue_12 (< _returnvalue_12 0.0))) (Math|Vector|ClampVectorSize (* (Math|Vector|GetRightVector _boomanchor) (Math|Float|SelectFloat (Math|Float|SelectFloat (- _returnvalue_12 (- _returnvalue_12 9e+01)) _returnvalue_12 (< 9e+01 _returnvalue_12)) (Math|Float|SelectFloat (- _returnvalue_12 (+ _returnvalue_12 9e+01)) _returnvalue_12 (< _returnvalue_12 -9e+01)) (< _returnvalue_12 0.0))) 0.0 1.0)))) _returnvalue_2) (Variables|Default|GetYawIntensity)))))