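; Sound manager actor that crossfades between day and night ambient audio as the time of day changes.
; On BeginPlay it finds BP_TimeOfDay, binds to its DayTime and NightTime events, stops the night track and sets both components to the configured Volume.
; Each event fades one AudioComponent in and the other out over FadeDuration.
; The construction script sets both components' volume multipliers to zero.
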(event Custom|DayTime_Event
  (Audio|Components|Audio|FadeIn (Variables|Default|GetAudioDay) (Variables|Default|GetFadeDuration) (Variables|Default|GetVolume) 0.0 "Linear" :!class /Script/Engine.AudioComponent)
  (Audio|Components|Audio|FadeOut (Variables|Default|GetAudioNight) (Variables|Default|GetFadeDuration) 0.0 "Linear" :!class /Script/Engine.AudioComponent))

(event Custom|NightTime_Event
  (Audio|Components|Audio|FadeIn (Variables|Default|GetAudioNight) (Variables|Default|GetFadeDuration) (Variables|Default|GetVolume) 0.0 "Linear" :!class /Script/Engine.AudioComponent)
  (Audio|Components|Audio|FadeOut (Variables|Default|GetAudioDay) (Variables|Default|GetFadeDuration) 0.0 "Linear" :!class /Script/Engine.AudioComponent))

(event EventBeginPlay
  (bind _volume (Variables|Default|GetVolume))
  (bind _returnvalue (Actor|GetActorOfClass "/Game/Blueprints/BP_TimeOfDay.BP_TimeOfDay_C"))
  (bind _output_get (Variables|Default|SetBP_TimeOfDay _returnvalue))
  (EventDispatchers|AssignDayTime _output_get (delegate Custom|DayTime_Event))
  (EventDispatchers|AssignNightTime _output_get (delegate Custom|NightTime_Event))
  (Audio|Components|Audio|Stop (Variables|Default|GetAudioNight))
  (Audio|Components|Audio|SetVolumeMultiplier (Variables|Default|GetAudioDay) _volume :!class /Script/Engine.AudioComponent)
  (Audio|Components|Audio|SetVolumeMultiplier (Variables|Default|GetAudioNight) _volume :!class /Script/Engine.AudioComponent))

(fn ConstructionScript
  (Audio|Components|Audio|SetVolumeMultiplier (Variables|Default|GetAudioDay) 0.0 :!class /Script/Engine.AudioComponent)
  (Audio|Components|Audio|SetVolumeMultiplier (Variables|Default|GetAudioNight) 0.0 :!class /Script/Engine.AudioComponent))