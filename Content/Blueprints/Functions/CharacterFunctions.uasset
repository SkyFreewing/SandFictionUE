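; Character function library that aligns a mesh to the ground beneath an actor and measures slope angle.
; Both functions trace a short line downward against one object type and use the impact normal.
; MatchGroundRotation interpolates mesh rotation toward the surface, keeping yaw and clamping roll, not pitch, by PitchAngle.
; CheckGroundAngle returns the difference between actor pitch and ground pitch.
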(fn MatchGroundRotation
  (params (Mesh :type Scene%20Component%20Object%20Reference) (Actor :type Actor%20Object%20Reference) (Pitch%20Angle :type Float%20%28single-precision%29) (InterpSpeed :type Float%20%28single-precision%29))
  (bind _returnvalue (Transformation|GetActorLocation Actor))
  (bind _returnvalue_2 (Transformation|GetWorldRotation Mesh))
  (bind (_outhit _returnvalue_3) (Collision|LineTraceForObjects 0 _returnvalue (- _returnvalue "0, 0,200.000000") (Utilities|Array|MakeArray "ObjectTypeQuery7") false 0 "None"))
  (if _returnvalue_3
    (Transformation|SetWorldRotation Mesh (Math|Interpolation|RInterpTo _returnvalue_2 (Math|Rotator|MakeRotator (Math|Float|Clamp(Float) (.Roll (Math|Rotator|BreakRotator (Math|Rotator|MakeRotfromXZ (Math|Vector|GetForwardVector Mesh) (.ImpactNormal (Collision|BreakHitResult _outhit))))) (* Pitch%20Angle -1.0) Pitch%20Angle) (.Pitch (Math|Rotator|BreakRotator (Class|KismetMathLibrary|MakeRotfromYZ (Math|Vector|GetRightVector Mesh) (.ImpactNormal (Collision|BreakHitResult _outhit))))) (.Yaw (Math|Rotator|BreakRotator _returnvalue_2))) (Utilities|Time|GetWorldDeltaSeconds) InterpSpeed) true false)
    (return (Math|Interpolation|RInterpTo _returnvalue_2 (Math|Rotator|MakeRotator (Math|Float|Clamp(Float) (.Roll (Math|Rotator|BreakRotator (Math|Rotator|MakeRotfromXZ (Math|Vector|GetForwardVector Mesh) (.ImpactNormal (Collision|BreakHitResult _outhit))))) (* Pitch%20Angle -1.0) Pitch%20Angle) (.Pitch (Math|Rotator|BreakRotator (Class|KismetMathLibrary|MakeRotfromYZ (Math|Vector|GetRightVector Mesh) (.ImpactNormal (Collision|BreakHitResult _outhit))))) (.Yaw (Math|Rotator|BreakRotator _returnvalue_2))) (Utilities|Time|GetWorldDeltaSeconds) InterpSpeed))))

(fn CheckGroundAngle
  (params (Actor :type Actor%20Object%20Reference))
  (bind _returnvalue (Transformation|GetActorLocation Actor))
  (bind (_outhit _returnvalue_2) (Collision|LineTraceForObjects 0 _returnvalue (- _returnvalue "0, 0,200.000000") (Utilities|Array|MakeArray "ObjectTypeQuery7") false 0 "None"))
  (if _returnvalue_2
    (return (- (.pitch (Transformation|GetActorRotation Actor)) (.Pitch (Math|Rotator|BreakRotator (Class|KismetMathLibrary|MakeRotfromYZ (Transformation|GetActorRightVector Actor) (.ImpactNormal (Collision|BreakHitResult _outhit)))))))))