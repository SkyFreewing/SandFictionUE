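; WaterDeadZone is a trigger volume that acts as a deep-water hazard, moving the player back onto navigable ground.
; Its Box overlap prints a debug message for any actor, then continues only for the player's MainCharacter_BP.
; It calls FadeToBlack on BP_TimeOfDay, waits briefly, then teleports the character to a random reachable navigation point around its current location, with no fixed respawn point.
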(event OnComponentBeginOverlap(Box)
  (params (OverlappedComponent :type Primitive%20Component%20Object%20Reference) (OtherActor :type Actor%20Object%20Reference) (OtherComp :type Primitive%20Component%20Object%20Reference) (OtherBodyIndex :type Integer) (bFromSweep :type Boolean) (SweepResult :type Hit%20Result%20Structure%20%28by%20ref%29))
  (bind _returnvalue (Game|GetPlayerCharacter 0))
  (bind _asmain_character_bp (Utilities|Casting|CastToMainCharacter_BP _returnvalue))
  (Development|PrintString "Player Enters Deep Water! Respawn!")
  (if (== OtherActor _asmain_character_bp)
    (bind _returnvalue_2 (Actor|GetActorOfClass "/Game/Blueprints/BP_TimeOfDay.BP_TimeOfDay_C"))
    (Default|FadetoBlack _returnvalue_2 5.0)
    (Utilities|FlowControl|Delay 1.0)
    (Transformation|SetActorLocation _asmain_character_bp (.RandomLocation (AI|Navigation|GetRandomReachablePointinRadius (Transformation|GetActorLocation _asmain_character_bp) 5e+02 0 0)) false true)))

(fn ConstructionScript)