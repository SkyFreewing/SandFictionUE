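; Base interactable container that opens the player menu with its own inventory when the player interacts with it.
; On BeginPlay it looks up each configured Items entry in its data table and adds it to the InventoryComponent.
; The construction script takes the UI description from the inventory name and refreshes preset inventory entries from their data table rows.
; An unconnected alternative would scatter the items as nearby actors and destroy the container.
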(event EventBeginPlay
  (|CallParentFunction)
  (for _array_element (Variables|Default|GetItems)
    (bind _returnvalue (Utilities|GetDataTableRow (.datatable (.datatableitem (.itemstructure _array_element))) (.rowname (.datatableitem (.itemstructure _array_element))))
      (:then
        (Default|AddtoInventory (Variables|Default|GetInventoryComponent) (Utilities|Struct|MakeInventorySlotStructure _returnvalue (.quantity _array_element)) false)))))

(event EventInteract
  (params (Player :type Main%20Character%20BP%20Object%20Reference))
  (|CallParentFunction 0)
  (bind _asmain_character_bp (Utilities|Casting|CastToMainCharacter_BP (Game|GetPlayerCharacter 0)))
  (bind _playermenu (Default|CreatePlayerMenu (.AsPlayer%20HUD%20BP (Utilities|Casting|CastToPlayerHUD_BP (HUD|GetHUD (Game|GetPlayerController 0)))) 4 _asmain_character_bp))
  (Default|ToggleInventory _playermenu (Variables|Default|GetInventoryComponent)))

(fn ConstructionScript
  (bind _inventorycomponent (Variables|Default|GetInventoryComponent))
  (bind _inventory (Variables|/Game/Blueprints/UI/Inventory/InventoryComponent.InventoryComponent_C|GetInventory _inventorycomponent))
  (|CallParentFunction)
  (Variables|Default|SetUIDescription (Variables|/Game/Blueprints/UI/Inventory/InventoryComponent.InventoryComponent_C|GetInventoryName _inventorycomponent))
  (for (_array_element _array_index) _inventory
    (bind _returnvalue (Utilities|GetDataTableRow (.datatable (.datatableitem (.ItemStructure (Utilities|Struct|BreakInventorySlotStructure _array_element)))) (.rowname (.datatableitem (.ItemStructure (Utilities|Struct|BreakInventorySlotStructure _array_element)))))
      (:then
        (Utilities|Array|SetArrayElem _inventory _array_index _returnvalue)))))