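; Storage_Corpse is a container Blueprint that, by its name, serves as the storage for a corpse.
; On BeginPlay it runs the parent logic, then sets its Storage slot count to match the Inventory of player 0's MainCharacter_BP.
; It adds no other active logic, as overlap and tick are disabled and construction only calls the parent.
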(event EventBeginPlay
  (|CallParentFunction)
  (Variables|/Game/Blueprints/UI/Inventory/InventoryComponent.InventoryComponent_C|SetNumberSlots (Variables|Default|GetStorage) (Variables|/Game/Blueprints/UI/Inventory/InventoryComponent.InventoryComponent_C|GetNumberSlots (Variables|/Game/Blueprints/Characters/MainCharacter/MainCharacter_BP.MainCharacter_BP_C|GetInventory (.AsMain%20Character%20BP (Utilities|Casting|CastToMainCharacter_BP (Game|GetPlayerCharacter 0)))))))

(event Collision|EventActorBeginOverlap
  (params (OtherActor :type Actor%20Object%20Reference))
  (|CallParentFunction OtherActor) ; This node is disabled and will not be called.\nDrag off pins to build functionality.
)

(event EventTick
  (params (DeltaSeconds :type Float%20%28single-precision%29))
  (|CallParentFunction DeltaSeconds) ; This node is disabled and will not be called.\nDrag off pins to build functionality.
)

(fn ConstructionScript
  (|CallParentFunction))