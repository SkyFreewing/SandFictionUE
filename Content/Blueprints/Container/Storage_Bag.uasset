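; Storage_Bag is a temporary container actor that holds items in a Storage component and removes itself from the world.
; On BeginPlay it copies its slot count from the player character's inventory and binds Despawn to the day-time event of BP_TimeOfDay, so that event destroys the bag.
; Every Tick it also scans the storage inventory and destroys itself once all slot quantities are zero.
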(event Custom|Despawn
  (Actor|DestroyActor))

(event EventBeginPlay
  (|CallParentFunction)
  (Variables|/Game/Blueprints/UI/Inventory/InventoryComponent.InventoryComponent_C|SetNumberSlots (Variables|Default|GetStorage) (Variables|/Game/Blueprints/UI/Inventory/InventoryComponent.InventoryComponent_C|GetNumberSlots (Variables|/Game/Blueprints/Characters/MainCharacter/MainCharacter_BP.MainCharacter_BP_C|GetInventory (.AsMain%20Character%20BP (Utilities|Casting|CastToMainCharacter_BP (Game|GetPlayerCharacter 0))))))
  (bind _returnvalue (Actor|GetActorOfClass "/Game/Blueprints/BP_TimeOfDay.BP_TimeOfDay_C"))
  (EventDispatchers|BindEventtoDayTime _returnvalue (delegate Custom|Despawn)))

(event EventTick
  (params (DeltaSeconds :type Float%20%28single-precision%29))
  (|CallParentFunction DeltaSeconds)
  (CallFunction|DestroywhenEmpty))

(fn ConstructionScript
  (|CallParentFunction))

(fn DestroywhenEmpty
  (bind _array_element (Utilities|Array|ForEachLoopwithBreak (Variables|/Game/Blueprints/UI/Inventory/InventoryComponent.InventoryComponent_C|GetInventory (Variables|Default|GetStorage)) :!label _label)
    (:LoopBody
      (if (== (.quantity _array_element) 0)
        (LocalVariables|SetEmpty true)
        (else
          (LocalVariables|SetEmpty false)
          (goto _label Break))))
    (:Completed
      (if (LocalVariables|GetEmpty)
        (Actor|DestroyActor)))))