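; Storage container variant that stocks itself with whole categories of items when play begins.
; On BeginPlay it scans the ItemList data table for each class in its ParentClass array and keeps rows whose item class derives from that class.
; Each match is added to the Storage inventory at its max stack size, with pickup creation suppressed.
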(event EventBeginPlay
  (|CallParentFunction)
  (for _array_element (Variables|Default|GetParentClass)
    (bind _outrownames (DataTable|GetDataTableRowNames "/Game/Blueprints/Items/ItemList.ItemList"))
    (for _array_element_2 _outrownames
      (bind _returnvalue (Utilities|GetDataTableRow "/Game/Blueprints/Items/ItemList.ItemList" _array_element_2)
        (:then
          (if (Utilities|ClassIsChildOf (.Class (Utilities|Struct|BreakItemStructure _returnvalue)) _array_element)
            (Default|AddtoInventory (Variables|Default|GetStorage) (Utilities|Struct|MakeInventorySlotStructure _returnvalue (.MaxStackSize (Utilities|Struct|BreakItemStructure _returnvalue))) true)))))))

(fn ConstructionScript
  (|CallParentFunction))