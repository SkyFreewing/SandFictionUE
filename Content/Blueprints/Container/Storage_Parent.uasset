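; Base Blueprint for interactable storage containers that hold an inventory the player can open.
; On BeginPlay it resolves each configured item through its data table row and adds the quantity to its Storage, suppressing pickup creation.
; Interacting creates the player menu through the HUD's interface manager on a preset tab and passes Storage to it.
; The construction script uses the inventory name as the UI description.
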(event EventBeginPlay
  (|CallParentFunction)
  (for _array_element (Variables|Default|GetItems)
    (bind _returnvalue (Utilities|GetDataTableRow (.datatable (.DataTableItem (Utilities|Struct|BreakItemStructure (.itemstructure _array_element)))) (.rowname (.DataTableItem (Utilities|Struct|BreakItemStructure (.itemstructure _array_element)))))
      (:then
        (Default|AddtoInventory (Variables|Default|GetStorage) (Utilities|Struct|MakeInventorySlotStructure _returnvalue (.quantity _array_element)) true)))))

(event EventInteract
  (params (Player :type Main%20Character%20BP%20Object%20Reference))
  (|CallParentFunction Player)
  (bind _playermenu (Default|CreatePlayerMenu (.AsPlayer%20Interface%20Manager%20BP (Utilities|Casting|CastToPlayerInterfaceManager_BP (HUD|GetHUD (Game|GetPlayerController 0)))) 4 Player))
  (Default|UpdateTab _playermenu (Variables|Default|GetStorage)))

(fn ConstructionScript
  (Variables|Default|SetUIDescription (Variables|/Game/Blueprints/UI/Inventory/InventoryComponent.InventoryComponent_C|GetInventoryName (Variables|Default|GetStorage)))
  (|CallParentFunction))