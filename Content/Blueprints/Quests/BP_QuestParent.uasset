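; Base quest Blueprint that child quests and tasks derive from, tracking whether a quest is active and done.
; On BeginPlay it caches the player's MainCharacter_BP and binds its empty Update event to the player's interact event.
; SetActive and FinishQuest store the Active and Done states.
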(event Custom|Update)

(event Custom|SetActive
  (params (Active :type Boolean))
  (CallFunction|OnSetActive Active))

(event Custom|FinishQuest
  (params (Yes :type Boolean))
  (Variables|Core|SetDone Yes))

(event EventBeginPlay
  (bind _asmain_character_bp (Utilities|Casting|CastToMainCharacter_BP (Game|GetPlayerCharacter 0)))
  (bind _output_get (Variables|Default|SetPlayerRef _asmain_character_bp))
  (EventDispatchers|BindEventtoInteract _output_get (delegate Custom|Update)))

(fn ConstructionScript)

(fn OnSetActive
  (params (Active :type Boolean))
  (Variables|Core|SetActive Active))