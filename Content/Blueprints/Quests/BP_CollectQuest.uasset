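; BP_CollectQuest is a quest Blueprint that tracks collecting a target number of a given item.
; On Update, it queries the player's inventory for the item and stores the total as the current piece count.
; It maps that count against the quest goal to a clamped 0–1 progress value and passes whether progress equals 1 to FinishQuest.
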(event EventBeginPlay
  (|CallParentFunction))

(event Collision|EventActorBeginOverlap
  (params (OtherActor :type Actor%20Object%20Reference))
  (|CallParentFunction OtherActor) ; This node is disabled and will not be called.\nDrag off pins to build functionality.
)

(event EventTick
  (params (DeltaSeconds :type Float%20%28single-precision%29))
  (|CallParentFunction DeltaSeconds) ; This node is disabled and will not be called.\nDrag off pins to build functionality.
)

(event EventUpdate
  (bind _amount (CallFunction|UpdateCurrentPieces))
  (CallFunction|UpdateProgress _amount))

(fn ConstructionScript
  (|CallParentFunction))

(fn UpdateProgress
  (params (Amount :type Integer))
  (bind _output_get (Variables|Default|SetQuestProgress (Math|Float|MapRangeClamped (Math|Conversions|ToFloat(Integer) Amount) 0.0 (Math|Conversions|ToFloat(Integer) (Variables|Default|GetQuestGoal)) 0.0 1.0)))
  (CallFunction|FinishQuest (== _output_get 1.0)))

(fn UpdateCurrentPieces
  (bind _totalamount (Default|InventoryQuery (Variables|/Game/Blueprints/Characters/MainCharacter/MainCharacter_BP.MainCharacter_BP_C|GetInventory (Variables|Default|GetPlayerRef)) (Variables|Default|GetItemToCollect) (Variables|Default|GetQuestGoal)))
  (bind _output_get (Variables|Default|SetCurrentPieces _totalamount))
  (return _output_get))