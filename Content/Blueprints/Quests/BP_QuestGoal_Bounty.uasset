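; BP_QuestGoal_Bounty is a quest goal that tracks bounty pieces toward a target count.
; IncrementCurrentBounty only raises the piece count, while the separate Update event recalculates progress.
; UpdateProgress maps the count against the goal to a clamped 0-1 value and passes whether it reached 1 to FinishQuestGoal.
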(event Custom|IncrementCurrentBounty
  (Math|Integer|IncrementInt (Variables|Default|GetCurrentPieces)))

(event EventBeginPlay
  (|CallParentFunction))

(event EventUpdate
  (CallFunction|UpdateProgress))

(fn ConstructionScript
  (|CallParentFunction))

(fn UpdateProgress
  (bind _output_get (Variables|Default|SetQuestProgress (Math|Float|MapRangeClamped (Math|Conversions|ToFloat(Integer) (Variables|Default|GetCurrentPieces)) 0.0 (Math|Conversions|ToFloat(Integer) (Variables|Default|GetQuestGoal)) 0.0 1.0)))
  (CallFunction|FinishQuestGoal (== _output_get 1.0)))