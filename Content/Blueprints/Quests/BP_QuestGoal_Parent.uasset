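; BP_QuestGoal_Parent is the base Blueprint for a single goal within a quest.
; On BeginPlay it takes the player reference from its ParentQuest and binds its empty Update event to the player's interact event.
; FinishQuestGoal marks the goal as done and calls DoWhenDone, which tells the parent quest to update its index.
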(event Custom|Update)

(event Custom|Finish%20Quest%20Goal
  (Variables|Core|SetGoalDone true)
  (CallFunction|DowhenDone))

(event Custom|DoWhenDone
  (Default|UpdateIndex (Variables|Default|GetParentQuest)))

(event EventBeginPlay
  (bind _output_get (Variables|Default|SetPlayerRef (Variables|/Game/Blueprints/Quests/BP_QuestParent.BP_QuestParent_C|GetPlayerRef (Variables|Default|GetParentQuest))))
  (EventDispatchers|BindEventtoInteract _output_get (delegate Custom|Update)))

(fn ConstructionScript)