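; BP_QuestGoal_Collect is a quest goal that tracks whether the player has collected a required number of a given item.
; On Update it queries the player's inventory for ItemToCollect and stores the total held as CurrentPieces.
; That count is mapped, clamped, against QuestGoal into a 0–1 QuestProgress, and FinishQuestGoal receives whether progress has reached full.
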(event EventUpdate
  (bind _amount (CallFunction|UpdateCurrentPieces))
  (CallFunction|UpdateProgress _amount))

(fn ConstructionScript
  (|CallParentFunction))

(fn UpdateProgress
  (params (Amount :type Integer))
  (bind _output_get (Variables|Default|SetQuestProgress (Math|Float|MapRangeClamped (Math|Conversions|ToFloat(Integer) Amount) 0.0 (Math|Conversions|ToFloat(Integer) (Variables|Default|GetQuestGoal)) 0.0 1.0)))
  (CallFunction|FinishQuestGoal (== _output_get 1.0)))

(fn UpdateCurrentPieces
  (bind _totalamount (Default|InventoryQuery (Variables|/Game/Blueprints/Characters/MainCharacter/MainCharacter_BP.MainCharacter_BP_C|GetInventory (Variables|Default|GetPlayerRef)) (Variables|Default|GetItemToCollect) (Variables|Default|GetQuestGoal)))
  (bind _output_get (Variables|Default|SetCurrentPieces _totalamount))
  (return _output_get))