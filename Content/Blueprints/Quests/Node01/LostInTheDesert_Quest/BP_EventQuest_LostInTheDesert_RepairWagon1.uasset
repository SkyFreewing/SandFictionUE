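; Quest event for repairing the first wagon in the Lost in the Desert quest, extending a parent event's completion logic.
; When done, it runs the parent behavior, then finds and destroys the broken Inaya cart actor.
; If that cart was found, it also enables the clothing station on the CaravanManager and refreshes the caravan status.
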(event EventBeginPlay
  (|CallParentFunction) ; This node is disabled and will not be called.\nDrag off pins to build functionality.
)

(event Collision|EventActorBeginOverlap
  (params (OtherActor :type Actor%20Object%20Reference))
  (|CallParentFunction OtherActor) ; This node is disabled and will not be called.\nDrag off pins to build functionality.
)

(event EventTick
  (params (DeltaSeconds :type Float%20%28single-precision%29))
  (|CallParentFunction DeltaSeconds) ; This node is disabled and will not be called.\nDrag off pins to build functionality.
)

(event EventDowhenDone
  (|CallParentFunction)
  (bind _returnvalue (Actor|GetActorOfClass "/Game/Blueprints/Caravan/InayaCart01_Broken.InayaCart01_Broken_C"))
  (Utilities|IsValid _returnvalue
    (:Is%20Valid
      (Actor|DestroyActor _returnvalue)
      (bind _returnvalue_2 (Actor|GetActorOfClass "/Game/Blueprints/Caravan/CaravanManager.CaravanManager_C"))
      (Variables|/Game/Blueprints/Caravan/CaravanManager.CaravanManager_C|SetClothingStation _returnvalue_2 true)
      (Default|UpdateCaravanStatus _returnvalue_2))))

(fn ConstructionScript
  (|CallParentFunction))