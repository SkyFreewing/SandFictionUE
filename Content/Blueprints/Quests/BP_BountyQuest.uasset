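; Bounty quest Blueprint that tracks a count of collected pieces against a goal and flags the quest as done.
; UpdateProgress adds an amount to CurrentPieces, sets QuestProgress to QuestGoal divided by CurrentPieces (the inverse of a usual progress ratio) clamped to 0–1, and calls FinishedQuest at exactly 1.
; The Update event calls UpdateProgress with zero, re-evaluating progress without adding pieces.
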(event EventBeginPlay
  (|CallParentFunction) ; This node is disabled and will not be called.\nDrag off pins to build functionality.
)

(event Collision|EventActorBeginOverlap
  (params (OtherActor :type Actor%20Object%20Reference))
  (|CallParentFunction OtherActor) ; This node is disabled and will not be called.\nDrag off pins to build functionality.
)

(event EventTick
  (params (DeltaSeconds :type Float%20%28single-precision%29))
  (|CallParentFunction DeltaSeconds) ; This node is disabled and will not be called.\nDrag off pins to build functionality.
)

(event EventUpdate
  (CallFunction|UpdateProgress))

(fn ConstructionScript
  (|CallParentFunction))

(fn UpdateProgress
  (params (Amount :type Integer))
  (bind _output_get (Variables|Default|SetCurrentPieces (+ Amount (Variables|Default|GetCurrentPieces))))
  (bind _output_get_2 (Variables|Default|SetQuestProgress (Math|Float|Clamp(Float) (/ (Math|Conversions|ToFloat(Integer) (Variables|Default|GetQuestGoal)) (Math|Conversions|ToFloat(Integer) _output_get)))))
  (if (== _output_get_2 1.0)
    (CallFunction|FinishedQuest)))

(fn FinishedQuest
  (Variables|Default|SetDone true))