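; Parent Blueprint actor for interactable objects that the main character can interact with.
; A sphere trigger registers and unregisters the actor with MainCharacter_BP on overlap, and ToggleHighlight shows or hides its prompt widget component.
; The construction script applies trigger radius and UI and trigger offsets from variables, and BeginPlay sets the prompt text.
; Interact and SetupMesh are empty hooks, apparently meant for child overrides.
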(event OnComponentBeginOverlap(InteractionTriggerComp)
  (params (OverlappedComponent :type Primitive%20Component%20Object%20Reference) (OtherActor :type Actor%20Object%20Reference) (OtherComp :type Primitive%20Component%20Object%20Reference) (OtherBodyIndex :type Integer) (bFromSweep :type Boolean) (SweepResult :type Hit%20Result%20Structure%20%28by%20ref%29))
  (bind _asmain_character_bp (Utilities|Casting|CastToMainCharacter_BP OtherActor))
  (bind _output_get (Variables|Interaction|SetPlayer _asmain_character_bp))
  (Default|AddInteraction _output_get self))

(event OnComponentEndOverlap(InteractionTriggerComp)
  (params (OverlappedComponent :type Primitive%20Component%20Object%20Reference) (OtherActor :type Actor%20Object%20Reference) (OtherComp :type Primitive%20Component%20Object%20Reference) (OtherBodyIndex :type Integer))
  (bind _asmain_character_bp (Utilities|Casting|CastToMainCharacter_BP OtherActor))
  (bind _output_get (Variables|Interaction|SetPlayer _asmain_character_bp))
  (Default|RemoveInteraction _output_get self))

(event EventBeginPlay
  (CallFunction|SetupUIText))

(fn ConstructionScript
  (CallFunction|SetupInteractionUI)
  (CallFunction|SetupInteractionTrigger)
  (CallFunction|SetupMesh))

(fn ToggleHighlight
  (params (Highlight :type Boolean))
  (Rendering|SetVisibility (Variables|UI|GetInteractionUIComp) Highlight false))

(fn Interact
  (params (Player :type Main%20Character%20BP%20Object%20Reference)))

(fn SetupInteractionUI
  (Transformation|SetRelativeLocation (Variables|UI|GetInteractionUIComp) (Variables|UI|GetUIOffset) false false))

(fn SetupInteractionTrigger
  (Components|Sphere|SetSphereRadius (Variables|Trigger|GetInteractionTriggerComp) (Variables|Trigger|GetTriggerRadius) true)
  (Transformation|SetRelativeLocation (Variables|Trigger|GetInteractionTriggerComp) (Variables|Trigger|GetTriggerOffset) false false))

(fn SetupMesh)

(fn SetupUIText
  (bind _aswbp_interact_ui (Utilities|Casting|CastToWBP_Interact_UI (UserInterface|GetUserWidgetObject (Variables|UI|GetInteractionUIComp))))
  (Default|SetInteractionText _aswbp_interact_ui (Variables|UI|GetUIDescription)))