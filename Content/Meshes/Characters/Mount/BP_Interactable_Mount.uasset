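; BP_Interactable_Mount is an interactable that lets the player mount up on a linked Mount.
; On Interact it runs the parent logic, then calls MountUp if the player is not already mounted.
; MountUp makes player controller 0 possess the Mount, disables player capsule, mesh and weapon collision, and snap-attaches the player to this actor's root.
; It flags the player as mounted and passes them to the Mount, whose reference is stored through GetMount.
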(event EventInteract
  (params (Player :type Main%20Character%20BP%20Object%20Reference))
  ;[1 1 1] Mounting
  (|CallParentFunction 0)
  (if (not (Variables|/Game/Meshes/Characters/MainCharacter/MainCharacter_BP.MainCharacter_BP_C|GetIsMounted Player))
    (CallFunction|MountUp Player)))

(fn ConstructionScript
  (|CallParentFunction))

(fn GetMount
  (params (Mount :type Mount%20BP%20Object%20Reference))
  (Variables|Default|SetMount Mount))

(fn MountUp
  (params (Player :type Main%20Character%20BP%20Object%20Reference))
  (Pawn|Possess (Game|GetPlayerController 0) (Variables|Default|GetMount))
  (Collision|SetCollisionEnabled (Variables|/Script/Engine.Character|GetCapsuleComponent Player) "NoCollision")
  (Transformation|AttachComponentToComponent (Variables|/Script/Engine.Actor|GetRootComponent Player) (Variables|Transformation|GetRootComponent) "None" "SnapToTarget" "SnapToTarget" "SnapToTarget" false)
  (Variables|/Game/Meshes/Characters/MainCharacter/MainCharacter_BP.MainCharacter_BP_C|SetIsMounted Player true)
  (Default|GetMountedPlayer (Variables|Default|GetMount) Player))