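; EnemyFur_BP is the Blueprint for a Fur enemy character, handling health bar visibility and movement speed.
; Every tick it measures the distance to the player character and shows the EnemyHealthbar component only while the player is within range.
; Walk and Run events switch the CharacterMovement max walk speed between a slow roaming pace and a faster pace for following the player.
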(event Custom|Walk
  ;[1 1 1] Set Walk / Run Speed for Roaming / Following the Player
  (Variables|/Script/Engine.CharacterMovementComponent|SetMaxWalkSpeed (Variables|Character|GetCharacterMovement) 1e+02))

(event Custom|Run
  ;[1 1 1] Set Walk / Run Speed for Roaming / Following the Player
  (Variables|/Script/Engine.CharacterMovementComponent|SetMaxWalkSpeed (Variables|Character|GetCharacterMovement) 5e+02))

(event EventTick
  (params (DeltaSeconds :type Float%20%28single-precision%29))
  (bind _enemyhealthbar (Variables|Default|GetEnemyHealthbar))
  ;[1 1 1] Only display Healthbar when in Range of the Player
  (if (< (Transformation|GetDistanceTo (Game|GetPlayerCharacter 0)) 1e+03)
    (Rendering|SetVisibility _enemyhealthbar true false)
    (else
      (Rendering|SetVisibility _enemyhealthbar false false))))

(fn ConstructionScript)