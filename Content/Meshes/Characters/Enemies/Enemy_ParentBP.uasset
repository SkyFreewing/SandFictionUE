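; Parent Blueprint for enemy characters, handling health display, death, lock-on visuals and movement speed.
; Tick pushes health to the EnemyHealthbar widget, destroys the actor when health is nearly zero, and shows the bar only near the player.
; TargetLockON toggles the target visual through a FlipFlop, while Walk and Run events switch max walk speed.
; A helper function returns the distance to the player.
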(event Custom|Walk
  ;[1 1 1] Set Walk / Run Speed for Roaming / Following the Player
  (Variables|/Script/Engine.CharacterMovementComponent|SetMaxWalkSpeed (Variables|Character|GetCharacterMovement) 1e+02))

(event Custom|Run
  ;[1 1 1] Set Walk / Run Speed for Roaming / Following the Player
  (Variables|/Script/Engine.CharacterMovementComponent|SetMaxWalkSpeed (Variables|Character|GetCharacterMovement) 5e+02))

(event EventTargetLockON
  (bind _targetvisual (Variables|Default|GetTargetVisual))
  ;[1 1 1] Only display Target Visual when in Range of the Player
  (Utilities|FlowControl|FlipFlop
    (:A
      (Development|SetHiddeninGame _targetvisual false false))
    (:B
      (Development|SetHiddeninGame _targetvisual true false))))

(event EventTick
  (params (DeltaSeconds :type Float%20%28single-precision%29))
  (bind _enemyhealthbar (Variables|Default|GetEnemyHealthbar))
  (bind _enemyhealth (Variables|Default|GetEnemyHealth))
  ;[1 1 1] Update Healthbar
  (bind _asenemy_healthbar (Utilities|Casting|CastToEnemyHealthbar (UserInterface|GetUserWidgetObject (Variables|Default|GetEnemyHealthbar))))
  (Variables|/Game/Meshes/Characters/Enemies/EnemyHealthbar.EnemyHealthbar_C|SetEnemyHealthPercentage _asenemy_healthbar _enemyhealth)
  (if (Math|Float|NearlyEqual(Float) _enemyhealth 0.0 1e-06)
    (Actor|DestroyActor)
    (else
      ;[1 1 1] Only display Healthbar when in Range of the Player
      (if (< (Transformation|GetDistanceTo (Game|GetPlayerCharacter 0)) 1e+03)
        (Rendering|SetVisibility _enemyhealthbar true false)
        (else
          (Rendering|SetVisibility _enemyhealthbar false false))))))

(fn ConstructionScript)

(fn DistancefromPlayerCheck
  (return (Transformation|GetDistanceTo (Game|GetPlayerCharacter 0))))